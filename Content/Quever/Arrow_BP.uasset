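; Arrow projectile fired by Enemy_ADC_BP that damages that shooter's MyEnemy target.
; One second after spawning, it caches the target and the Instigator's forward vector, then starts the Delete timeline that destroys it when finished.
; Tick moves it along that vector at a frame-rate-dependent step without sweeping.
; Any HitBox overlap destroys it, but only the target takes damage and clears the shooter's CanHitR flag.
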(event OnComponentBeginOverlap(hitBox)
  (params (OverlappedComponent :type Primitive%20Component%20Object%20Reference) (OtherActor :type Actor%20Object%20Reference) (OtherComp :type Primitive%20Component%20Object%20Reference) (OtherBodyIndex :type Integer) (bFromSweep :type Boolean) (SweepResult :type Hit%20Result%20Structure%20%28by%20ref%29))
  (if (== OtherActor (Variables|Default|GetMyEnemy))
    (Variables|/Game/Monster/AI/Parent/Enemy_BP.Enemy_BP_C|SetCanHit_R (.AsEnemy%20ADC%20BP (Utilities|Casting|CastToEnemy_ADC_BP (Variables|Actor|GetInstigator))) false)
    (Default|TakeDamage (Variables|Default|GetMyEnemy) 1e+01)
    (Actor|DestroyActor)
    (else
      (Actor|DestroyActor))))

(event EventBeginPlay
  (Utilities|FlowControl|Delay 1.0)
  (Variables|Default|SetMyEnemy (Variables|/Game/Monster/AI/Parent/Enemy_BP.Enemy_BP_C|GetMy%20Enemy (.AsEnemy%20ADC%20BP (Utilities|Casting|CastToEnemy_ADC_BP (Variables|Actor|GetInstigator)))))
  (Variables|Default|SetMyVector (Transformation|GetActorForwardVector (Variables|Actor|GetInstigator)))
  (Timeline|Delete PlayFromStart
    (:Finished
      (Actor|DestroyActor))))

(event Collision|EventActorBeginOverlap
  (params (OtherActor :type Actor%20Object%20Reference)))

(event EventTick
  (params (DeltaSeconds :type Float%20%28single-precision%29))
  (Transformation|AddActorWorldOffset (* (Variables|Default|GetMyVector) 5e+01)))

(fn ConstructionScript)