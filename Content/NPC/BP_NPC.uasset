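; Shopkeeper NPC that opens a shop screen when the player character overlaps its ShopTrigger.
; The overlap blends the view to the NPC, shows the mouse cursor and hides the player and their weapon.
; After a delay matching the blend, it creates a ShopKeeper_UI linked to itself, stores it, focuses it and disables character input.
; Closing the shop and restoring the player are not handled here.
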(event OnComponentBeginOverlap(ShopTrigger)
  (params (OverlappedComponent :type Primitive%20Component%20Object%20Reference) (OtherActor :type Actor%20Object%20Reference) (OtherComp :type Primitive%20Component%20Object%20Reference) (OtherBodyIndex :type Integer) (bFromSweep :type Boolean) (SweepResult :type Hit%20Result%20Structure%20%28by%20ref%29))
  (bind _returnvalue (Game|GetPlayerController 0))
  (bind _asthird_person_character (Utilities|Casting|CastToThirdPersonCharacter OtherActor))
  (if (== OtherActor (Game|GetPlayerCharacter 0))
    (Game|Player|SetViewTargetwithBlend (Game|GetPlayerController 0) self 0.7 "VTBlend_Linear" 0.0 false)
    (Input|SetInputModeGameandUI _returnvalue 0 "DoNotLock" true)
    (Variables|/Script/Engine.PlayerController|SetbShowMouseCursor _returnvalue true)
    (Rendering|SetActorHiddenInGame (Game|GetPlayerCharacter 0) true)
    (Rendering|SetActorHiddenInGame (Variables|/Game/ThirdPersonCPP/Blueprints/ThirdPersonCharacter.ThirdPersonCharacter_C|GetPlayerWeapon _asthird_person_character) true)
    (Utilities|FlowControl|Delay 0.7)
    (bind _returnvalue_2 (UserInterface|CreateWidget "/Game/NPC/ShopKeeper_UI.ShopKeeper_UI_C" (Game|GetPlayerController 0) self))
    (CallFunction|ShopWidget _returnvalue_2)
    (UserInterface|Viewport|AddtoViewport _returnvalue_2 0)
    (Input|SetInputModeGameandUI (Game|GetPlayerController 0) _returnvalue_2 "DoNotLock" true)
    (Input|DisableInput (Game|GetPlayerCharacter 0) (Game|GetPlayerController 0))))

(fn ConstructionScript)

(fn ShopWidget
  (params (ShopWidget :type User%20Widget%20Object%20Reference))
  (Variables|Default|Setshop_Widget ShopWidget))