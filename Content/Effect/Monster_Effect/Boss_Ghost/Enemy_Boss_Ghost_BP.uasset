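; Phase-two ghost of the boss that performs a single skill against the player, then fades out and destroys itself.
; On BeginPlay, the instigating boss's Phase2GhostSkill sets the skill, delay and, in some cases, facing.
; Each skill plays a montage whose notifies spawn AOE actors, then spawn attacks or enable SkillBody collision, except thunder, which uses a timeline.
; SkillBody overlaps damage the player according to the current montage section.
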(event OnComponentBeginOverlap(SKillBody)
  (params (OverlappedComponent :type Primitive%20Component%20Object%20Reference) (OtherActor :type Actor%20Object%20Reference) (OtherComp :type Primitive%20Component%20Object%20Reference) (OtherBodyIndex :type Integer) (bFromSweep :type Boolean) (SweepResult :type Hit%20Result%20Structure%20%28by%20ref%29))
  (bind _mesh (Variables|Character|GetMesh))
  (bind _myenemy_g (Variables|Default|GetMyEnemy_G))
  (bind _returnvalue (Transformation|GetActorTransform _myenemy_g))
  (bind _returnvalue_2 (Components|SkeletalMesh|GetAnimInstance _mesh))
  (switch name (Animation|Montage|MontageGetCurrentSection _returnvalue_2 (Animation|Montage|GetCurrentActiveMontage _returnvalue_2))
    (:Attack
      (Default|TakeDamage (Variables|Default|GetMyEnemy_G) 5e+01))
    (:Dash
      (Transformation|SetActorTransform _myenemy_g (Math|Transform|MakeTransform (.location _returnvalue) (Math|Conversions|RotationFromXVector (* (Math|Vector|GetForwardVector (Transformation|GetActorRotation)) -1.0)) (.scale _returnvalue)))
      (Animation|Montage|PlayMontage (Variables|/Script/Engine.Character|GetMesh _myenemy_g) "/Game/Player_Taunt_Montage.Player_Taunt_Montage"
        (:then
          (Default|TakeDamage (Variables|Default|GetMyEnemy_G) 3e+01))))
    (:Spin
      (Default|TakeDamage (Variables|Default|GetMyEnemy_G) 5e+01)
      (Transformation|SetRelativeScale3D (Variables|Default|GetSKillBody) "3.000000,3.000000,3.000000"))))

(event Event경직
  (params (DamageSize :type Float%20%28single-precision%29)))

(event Event경직끝)

(event EventBeginPlay
  (bind _returnvalue (Transformation|GetActorTransform))
  (bind _returnvalue_2 (Transformation|GetActorTransform))
  (bind _returnvalue_3 (Transformation|GetActorTransform))
  (bind _returnvalue_4 (Transformation|GetActorTransform))
  (bind _returnvalue_5 (Transformation|GetActorForwardVector))
  (bind _returnvalue_6 (Transformation|GetActorLocation))
  (bind _self self)
  (bind _returnvalue_7 (* _returnvalue_5 2e+02))
  (bind _returnvalue_8 (+ _returnvalue_7 (.location _returnvalue_4)))
  (Variables|/Script/Engine.CharacterMovementComponent|SetMaxWalkSpeed (Variables|Character|GetCharacterMovement) 1.2e+03)
  (bind _asthird_person_character (Utilities|Casting|CastToThirdPersonCharacter (Game|GetPlayerCharacter 0)))
  (Variables|Default|SetMyEnemy_G _asthird_person_character)
  (Collision|SetCollisionEnabled (Variables|Default|GetSKillBody) "NoCollision")
  (bind _asenemy_boss_bp (Utilities|Casting|CastToEnemy_Boss_BP (Variables|Default|GetInstigator)))
  (switch int (Variables|/Game/Monster/AI/Boss/Enemy_Boss_BP.Enemy_Boss_BP_C|GetPhase2GhostSkill _asenemy_boss_bp)
    (:0
      (Variables|Default|SetSkillInt 5)
      (Utilities|FlowControl|Delay 3.0)
      (Pawn|UnPossess (Pawn|GetController))
      (Transformation|SetActorRotation (Math|Rotator|FindLookatRotation (Transformation|GetActorLocation) (Math|Vector|MakeVector 4e+02 8e+02 378.019043))))
    (:1
      (Variables|Default|SetSkillInt (Variables|/Game/Monster/AI/Boss/Enemy_Boss_BP.Enemy_Boss_BP_C|GetSkillInt _asenemy_boss_bp))
      (Utilities|FlowControl|Delay 0.5))
    (:2
      (Variables|Default|SetSkillInt 3)
      (Utilities|FlowControl|Delay 3.0)
      (Transformation|SetActorRotation (Math|Rotator|FindLookatRotation (Math|Vector|MakeVector (.x _returnvalue_6) (.y _returnvalue_6) (.z _returnvalue_6)) (Transformation|GetActorLocation (Variables|Default|GetMyEnemy_G))))
      (Utilities|FlowControl|Delay 1.0))
    (:3
      (Variables|Default|SetSkillInt 1)
      (Utilities|FlowControl|Delay 3.0)
      (Pawn|UnPossess (Pawn|GetController))
      (Transformation|SetActorRotation (Math|Rotator|FindLookatRotation (Transformation|GetActorLocation) (Math|Vector|MakeVector 6e+02 8e+02 378.019043))))
    (:4
      (Variables|Default|SetSkillInt (Variables|/Game/Monster/AI/Boss/Enemy_Boss_BP.Enemy_Boss_BP_C|GetSkillInt _asenemy_boss_bp))
      (Utilities|FlowControl|Delay 2.0)))
  (switch int (Variables|Default|GetSkillInt)
    (:0
      ;[1 1 1] 저돌맹진
      (Animation|Montage|PlayMontage (Variables|Character|GetMesh) "/Game/Monster/AI/Boss/SkillType/Dash_Boss.Dash_Boss" 1.2
        (:OnCompleted
          (Collision|SetCollisionEnabled (Variables|Default|GetSkillBody) "NoCollision" :!label _label)
          (bind _새_트랙_0 (Timeline|타임라인_0 PlayFromStart)
            (:Update
              (Utilities|FlowControl|Sequence
                (:then_0
                  (Rendering|Material|SetScalarParameterValueonMaterials (Variables|Character|GetMesh) "Opacity" _새_트랙_0))
                (:then_1
                  (Rendering|Material|SetScalarParameterValueonMaterials (Variables|Default|GetSickle_R) "Opacity" _새_트랙_0))
                (:then_2
                  (Rendering|Material|SetScalarParameterValueonMaterials (Variables|Default|GetSickle_L) "Opacity" _새_트랙_0))))
            (:Finished
              (Utilities|FlowControl|Delay 1.0)
              (Actor|DestroyActor))))
        (:OnInterrupted
          (goto _label))
        (:OnNotifyBegin
          (bind _returnvalue_9 (Game|SpawnActorfromClass "/Game/Monster/AI/Boss/SkillType/Skill/DashAttack_AOE.DashAttack_AOE_C" (Math|Transform|MakeTransform _returnvalue_8 (.rotation _returnvalue_4) (+ _returnvalue_8 "0, 0,-100.000000")) "Undefined" 0 self)))
        (:OnNotifyEnd
          (Collision|SetCollisionEnabled (Variables|Default|GetSkillBody) "QueryOnly")
          (Actor|DestroyActor _returnvalue_9))))
    (:1
      ;[1 1 1] 탈태
      (Transformation|SetRelativeScale3D (Variables|Default|GetSkillBody) "30.000000,30.000000,30.000000")
      (Animation|Montage|PlayMontage (Variables|Character|GetMesh) "/Game/Monster/AI/Boss/SkillType/Spin_Boss.Spin_Boss" 0.8
        (:OnCompleted
          (goto _label))
        (:OnInterrupted
          (goto _label))
        (:OnNotifyBegin
          (bind _returnvalue_10 (Game|SpawnActorfromClass "/Game/Monster/AI/Boss/SkillType/Skill/SpinAttack2_AOE.SpinAttack2_AOE_C" (Math|Transform|MakeTransform (+ (.location _returnvalue_2) "0, 0,-100.000000") (.rotation _returnvalue_2) (.scale _returnvalue_2)) "Undefined" 0 0)))
        (:OnNotifyEnd
          (Utilities|FlowControl|Delay 1.0)
          (Actor|DestroyActor _returnvalue_10)
          (Collision|SetCollisionEnabled (Variables|Default|GetSkillBody) "QueryOnly")
          (Utilities|FlowControl|Delay 0.1)
          (Collision|SetCollisionEnabled (Variables|Default|GetSkillBody) "NoCollision"))))
    (:2
      ;[1 1 1] 천둥호출
      (Animation|Montage|PlayMontage (Variables|Character|GetMesh) "/Game/Monster/AI/Boss/Boss_Cast_Montage.Boss_Cast_Montage" 1.2
        (:OnCompleted
          (goto _label))
        (:OnInterrupted
          (goto _label))
        (:OnNotifyBegin
          (Timeline|타임라인_1 PlayFromStart
            (:Thunder
              (bind _output_get (Variables|Default|SetplayerTransform (Transformation|GetActorTransform (Variables|Default|GetMyEnemy_G))))
              (Game|SpawnActorfromClass "/Game/Monster/AI/Boss/SkillType/Skill/ThunderAttack_AOE.ThunderAttack_AOE_C" (Math|Transform|MakeTransform (+ (.location _output_get) "0, 0,-100.000000") (.rotation _output_get) (.scale _output_get)) "Undefined" 0 0))))))
    (:3
      ;[1 1 1] 일섬
      (Animation|Montage|PlayMontage (Variables|Character|GetMesh) "/Game/Monster/AI/Boss/SkillType/Cast_Montage.Cast_Montage" 1.2
        (:OnCompleted
          (goto _label))
        (:OnInterrupted
          (goto _label))
        (:OnNotifyBegin
          (bind _returnvalue_11 (Game|SpawnActorfromClass "/Game/Monster/AI/Boss/SkillType/Skill/RailAttack_AOE.RailAttack_AOE_C" (Math|Transform|MakeTransform (+ (+ (* (Transformation|GetActorForwardVector) 2e+02) (.location _returnvalue)) "0, 0,-100.000000") (.rotation _returnvalue) "1,1,1") "Undefined" 0 self)))
        (:OnNotifyEnd
          (Game|SpawnActorfromClass "/Game/Monster/AI/Boss/SkillType/Skill/RailAttack.RailAttack_C" (Math|Transform|MakeTransform (+ (* (Math|Vector|GetForwardVector (Variables|/Game/Monster/AI/Boss/SkillType/Skill/RailAttack_AOE.RailAttack_AOE_C|GetPlane _returnvalue_11)) -8e+02) (.location (Transformation|GetActorTransform _returnvalue_11))) (.rotation (Transformation|GetActorTransform _returnvalue_11)) "1,1,1") "Undefined" 0 0)
          (Actor|DestroyActor _returnvalue_11))))
    (:4
      ;[1 1 1] 방전
      (Animation|Montage|PlayMontage (Variables|Character|GetMesh) "/Game/Monster/AI/Boss/Standing_Taunt_Battlecry_Montage.Standing_Taunt_Battlecry_Montage" 1.2
        (:OnCompleted
          (goto _label))
        (:OnInterrupted
          (goto _label))
        (:OnNotifyBegin
          (bind _returnvalue_12 (Game|SpawnActorfromClass "/Game/Monster/AI/Boss/SkillType/Skill/AroundAttack_AOE.AroundAttack_AOE_C" (Math|Transform|MakeTransform (+ (.location _returnvalue_3) "0, 0,-100.000000") (.rotation _returnvalue_3) "30.000000,30.000000,30.000000") "Undefined" 0 0)))
        (:OnNotifyEnd
          (Game|SpawnActorfromClass "/Game/Monster/AI/Boss/SkillType/Skill/AroundAttack.AroundAttack_C" (Math|Transform|MakeTransform (.location _returnvalue_3) (.rotation _returnvalue_3) "30.000000,30.000000,30.000000") "Undefined" 0 0)
          (Actor|DestroyActor _returnvalue_12))))
    (:5
      ;[1 1 1] 휩쓸기
      (Variables|Default|SetMytransform_G (Transformation|GetActorTransform))
      (Animation|Montage|PlayMontage (Variables|Character|GetMesh) "/Game/Monster/AI/Boss/SkillType/Brush_Boss.Brush_Boss" 1.2
        (:OnCompleted
          (goto _label))
        (:OnInterrupted
          (goto _label))
        (:OnNotifyBegin
          (bind _returnvalue_13 (Game|SpawnActorfromClass "/Game/Monster/AI/Boss/SkillType/Skill/PizzaAttack_AOE.PizzaAttack_AOE_C" (Math|Transform|MakeTransform (+ (.location _returnvalue_3) "0, 0,-90.000000") (Math|Rotator|MakeRotator 0.0 0.0 (+ (.Yaw (Math|Rotator|BreakRotator (.rotation _returnvalue_3))) 1.8e+02)) "10.000000,10.000000,1") "Undefined" 0 0)))
        (:OnNotifyEnd
          (Game|SpawnActorfromClass "/Game/Monster/AI/Boss/SkillType/Skill/PizzaAttack_R.PizzaAttack_R_C" (Math|Transform|MakeTransform (.location (Variables|Default|GetMytransform_G)) (.rotation (Variables|Default|GetMytransform_G)) "1.500000,1.000000,1.000000") "Undefined" 0 _self)
          (Game|SpawnActorfromClass "/Game/Monster/AI/Boss/SkillType/Skill/PizzaAttack_L.PizzaAttack_L_C" (Math|Transform|MakeTransform (.location (Variables|Default|GetMytransform_G)) (.rotation (Variables|Default|GetMytransform_G)) "1.500000,1.000000,1") "Undefined" 0 _self)
          (Actor|DestroyActor _returnvalue_13))))))

(fn ConstructionScript
  (|CallParentFunction))