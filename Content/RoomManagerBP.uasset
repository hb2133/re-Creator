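; Room manager actor that starts enemy spawning in the player's current room and resets its exit triggers.
; It registers a callback with ThirdPersonCharacter, which acts only while the Box overlap flags the room as current.
; The callback starts, once, the spawner whose ActivationID matches the parent actor's name, and hides the manager.
; It immediately calls RoomClearCall, clearing IsUsed on Up, Right and Left triggers and restoring visibility and collision.
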(event OnComponentBeginOverlap(Box)
  (params (OverlappedComponent :type Primitive%20Component%20Object%20Reference) (OtherActor :type Actor%20Object%20Reference) (OtherComp :type Primitive%20Component%20Object%20Reference) (OtherBodyIndex :type Integer) (bFromSweep :type Boolean) (SweepResult :type Hit%20Result%20Structure%20%28by%20ref%29))
  (Utilities|Casting|CastToThirdPersonCharacter OtherActor)
  (Variables|Default|SetCurrentRoom true))

(event OnComponentEndOverlap(Box)
  (params (OverlappedComponent :type Primitive%20Component%20Object%20Reference) (OtherActor :type Actor%20Object%20Reference) (OtherComp :type Primitive%20Component%20Object%20Reference) (OtherBodyIndex :type Integer))
  (Variables|Default|SetCurrentRoom false))

(event Custom|ActivateSpawner
  (params (Activation_ID :type String))
  ;[1 1 1] 스폰
  (bind _outactors (Actor|GetAllActorsOfClass "/Game/Monster/Levels/Enemy_Spawner_BP.Enemy_Spawner_BP_C"))
  (bind _array_element (Utilities|Array|ForEachLoopwithBreak _outactors :!label _label)
    (:LoopBody
      (if (Utilities|Enum|Equal(Enum) (Variables|/Game/Monster/Levels/Enemy_Spawner_BP.Enemy_Spawner_BP_C|GetActivation_ID _array_element) Activation_ID)
        (goto _label Break)))
    (:Completed
      (Utilities|FlowControl|DoOnce false
        (:Completed
          (Default|StartSpawning _array_element))))))

(event Custom|RoomManagerCall_Event_0
  (if (Variables|Default|GetCurrentRoom)
    (CallFunction|ActivateSpawner (Utilities|GetObjectName (Actor|GetAttachParentActor)))
    (Variables|Default|SetisPlaying true)
    (Rendering|SetActorHiddenInGame true)
    (Collision|SetCollisionEnabled (Variables|Default|GetStaticMesh) "NoCollision")
    (CallFunction|RoomClearCall)))

(event Custom|RoomClearCall
  (bind _inforoom (Variables|Default|GetInfoRoom))
  (bind (_up _down _right _left) (Utilities|Struct|BreakDirect _inforoom))
  (bind _asroom_trigger (Utilities|Casting|CastToRoomTrigger (.nextMapTrigger (Utilities|Struct|BreakRoomNode _up))))
  (Variables|/Game/Level/RoomTrigger.RoomTrigger_C|SetisUsed _asroom_trigger false)
  (bind _asroom_trigger_2 (Utilities|Casting|CastToRoomTrigger (.nextMapTrigger (Utilities|Struct|BreakRoomNode _right))))
  (Variables|/Game/Level/RoomTrigger.RoomTrigger_C|SetisUsed _asroom_trigger_2 false)
  (bind _asroom_trigger_3 (Utilities|Casting|CastToRoomTrigger (.nextMapTrigger (Utilities|Struct|BreakRoomNode _left))))
  (Variables|/Game/Level/RoomTrigger.RoomTrigger_C|SetisUsed _asroom_trigger_3 false)
  (Rendering|SetActorHiddenInGame false)
  (Collision|SetCollisionEnabled (Variables|Default|GetStaticMesh) "QueryAndPhysics"))

(event EventBeginPlay
  (bind _asthird_person_character (Utilities|Casting|CastToThirdPersonCharacter (Game|GetPlayerCharacter 0)))
  (EventDispatchers|AssignRoomManagerCall _asthird_person_character (delegate Custom|RoomManagerCall_Event_0)))

(event Collision|EventActorBeginOverlap
  (params (OtherActor :type Actor%20Object%20Reference)))

(event EventTick
  (params (DeltaSeconds :type Float%20%28single-precision%29)))

(fn ConstructionScript)