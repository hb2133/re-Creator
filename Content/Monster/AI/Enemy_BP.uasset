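; Skeleton melee enemy that chases the player character, attacks with a socket-attached sword and drops coins on death.
; A delay-retry AIMoveTo loop drives pursuit, while the AttackRange overlap repeats attack montages and sword overlap deals gated damage.
; 경직 applies damage and freezes a random hit-reaction pose with shake and sound until 경직끝 releases it.
; Death spawns loot and destroys enemy and weapon after a random delay; ragdoll is a separate event.
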(event OnComponentBeginOverlap(AttackRange)
  (params (OverlappedComponent :type Primitive%20Component%20Object%20Reference) (OtherActor :type Actor%20Object%20Reference) (OtherComp :type Primitive%20Component%20Object%20Reference) (OtherBodyIndex :type Integer) (bFromSweep :type Boolean) (SweepResult :type Hit%20Result%20Structure%20%28by%20ref%29))
  (if (and (== OtherActor (Variables|Default|GetMy%20Enemy)) (not (Variables|Default|GetIsAttacking)))
    (Variables|Default|SetCanAttack true :!label _label)
    (Variables|Default|SetIsAttacking true :!label _label_2)
    (Animation|Montage|PlayMontage (Variables|Character|GetMesh) "/Game/Monster/AI/Corpse_Alert_Attack_Fast2_Montage.Corpse_Alert_Attack_Fast2_Montage"
      (:OnCompleted
        _)
      (:OnInterrupted
        _))
    (Variables|Default|SetIsAttacking false)
    (if (Math|Boolean|ANDBoolean (Variables|Default|GetCanAttack) (Variables|Default|GetIsAlive) (not (Variables|Default|GetisDamaged)))
      (goto _label_2)
      (else
        (Utilities|FlowControl|Delay 0.7)
        (if (stale OnComponentEndOverlap(AttackRange) _output_get)
          (goto _label))))))

(event OnComponentEndOverlap(AttackRange)
  (params (OverlappedComponent :type Primitive%20Component%20Object%20Reference) (OtherActor :type Actor%20Object%20Reference) (OtherComp :type Primitive%20Component%20Object%20Reference) (OtherBodyIndex :type Integer))
  (if (and (== OtherActor (Variables|Default|GetMy%20Enemy)) (Variables|Default|GetCanAttack))
    (bind _output_get (Variables|Default|SetCanAttack false))))

(event OnComponentBeginOverlap(SwordCollision_R)
  (params (OverlappedComponent :type Primitive%20Component%20Object%20Reference) (OtherActor :type Actor%20Object%20Reference) (OtherComp :type Primitive%20Component%20Object%20Reference) (OtherBodyIndex :type Integer) (bFromSweep :type Boolean) (SweepResult :type Hit%20Result%20Structure%20%28by%20ref%29))
  (if (and (== OtherActor (Variables|Default|GetMy%20Enemy)) (Variables|Default|GetCanHit_R))
    (Variables|Default|SetCanHit_R false)
    (Default|TakeDamage (Variables|Default|GetMy%20Enemy) 5e+01)))

(event Custom|GetEnemy
  ;[1 1 1] AI
  (Utilities|FlowControl|Delay 1.0)
  (bind _outactors (Actor|GetAllActorsOfClass "/Game/ThirdPersonCPP/Blueprints/ThirdPersonCharacter.ThirdPersonCharacter_C"))
  (Variables|Default|SetMy%20Enemy (Utilities|Array|Get(acopy) _outactors)))

(event Custom|BaseMovement
  ;[1 1 1] AI
  (Utilities|IsValid (Variables|Default|GetMy%20Enemy) :!label _label
    (:Is%20Valid
      (if (Variables|Default|GetIsAlive)
        (if (Variables|Default|GetisDamaged)
          _
          (else
            (AI|AIMoveTo self "0, 0, 0" (Variables|Default|GetMy%20Enemy) 75.0 false
              (:OnSuccess
                _)
              (:OnFail
                (goto _label)))))
        ;;[1 1 1] 공격후 정지시간
        (Utilities|FlowControl|Delay 0.1)
        (goto _label)))
    (:Is%20Not%20Valid
      ;;[1 1 1] Nav시작시간
      (Utilities|FlowControl|Delay 0.1)
      (goto _label))))

(event Custom|TakeDamage
  (params (Amount :type Float%20%28single-precision%29))
  (bind _output_get (Variables|Default|SetHealth (- (Variables|Default|GetHealth) Amount)))
  (if (> _output_get 0.0)
    (Development|PrintString (Utilities|String|ToString(Float) (Variables|Default|GetHealth)) true true "(R=1.000000,G=0.000000,B=0.026892,A=1.000000)")
    (else
      (CallFunction|Die))))

(event Custom|Die
  (Variables|Default|SetIsAlive false)
  (Audio|PlaySound2D "/Game/Sound/202091__spookymodem__falling-bones-해골_사망.202091__spookymodem__falling-bones-해골_사망" 1.0 1.0 0.0 0 0)
  (Audio|PlaySound2D "/Game/Sound/614315__scorpion67890__gnasher-death-해골사망2.614315__scorpion67890__gnasher-death-해골사망2" 1.0 1.0 0.0 0 0)
  (Components|Movement|StopMovementImmediately (Variables|Character|GetCharacterMovement))
  (AI|ClearFocus (Variables|Default|GetAIController))
  (for _index (range 3 5)
    (CallFunction|DropLoot))
  (Utilities|FlowControl|Delay (Math|Conversions|ToFloat(Integer) (Math|Random|RandomIntegerinRange 4 6)))
  (Actor|DestroyActor)
  (Actor|DestroyActor (Variables|Default|GetEnemy_Weapon)))

(event Custom|StartRagdoll
  (bind _mesh (Variables|Character|GetMesh))
  (Class|SkeletalMeshComponent|SetAllBodiesSimulatePhysics _mesh true)
  (Collision|SetCollisionProfileName _mesh "Ragdoll" true :!class /Script/Engine.PrimitiveComponent)
  (Collision|SetCollisionEnabled (Variables|Collision|GetCapsuleComponent) "NoCollision"))

(event Custom|경직
  (params (DamageSize :type Float%20%28single-precision%29))
  (CallFunction|GetDamage DamageSize)
  (Variables|Default|SetisDamaged true)
  (Components|Movement|StopMovementImmediately (Variables|Character|GetCharacterMovement))
  (Animation|Montage|PlayMontage (Variables|Character|GetMesh) "/Game/CityofBrass_Enemies/Meshes/Enemy/Corpse/animation/Monster_Damaged.Monster_Damaged" 0.0 0.0 (Utilities|String|StringToName (Utilities|String|ToString(Integer) (Class|KismetMathLibrary|RandomIntegerfromStream 4 (Variables|Default|GetRandomAnimation))))
    (:then
      (Class|MatineeCameraShake|StartMatineeCameraShake (Game|GetPlayerCameraManager 0) "/Game/Camera/Shake.Shake_C" 0.05 "CameraLocal" "0, 0, 0")
      (Audio|PlaySound2D "/Game/Sound/202091_spookymodem_falling-bones-해골_피격2.202091_spookymodem_falling-bones-해골_피격2" 1.0 1.0 0.0 0 0)
      (Audio|PlaySound2D "/Game/Sound/Ice_Impact_Throw_Snowball_Step_Snow_Stalactite_Various12_M-해골_피격.Ice_Impact_Throw_Snowball_Step_Snow_Stalactite_Various12_M-해골_피격" 1.0 1.0 0.0 0 0))))

(event Custom|경직끝
  (Animation|Montage|PlayMontage (Variables|Character|GetMesh) "/Game/CityofBrass_Enemies/Meshes/Enemy/Corpse/animation/Monster_Damaged.Monster_Damaged" 5.0 0.0 "action"
    (:OnCompleted
      _)
    (:OnInterrupted
      (Development|PrintString "몽타주 멈춤!")))
  (Variables|Default|SetisDamaged false))

(event Custom|Drop%20Loot
  (bind _returnvalue (Transformation|GetActorLocation))
  ;[1 1 1] 몬스터의 아이템 드랍
  (bind _outhit (Collision|LineTraceByChannel _returnvalue (- _returnvalue "0, 0,200.000000") "TraceTypeQuery1" false (Utilities|Array|MakeArray (Game|GetPlayerCharacter 0)) "None"))
  (bind _returnvalue_2 (Game|SpawnActorfromClass (Utilities|Select :Index (Math|Random|RandomInteger 5) :Option%200 "/Game/Coin/Coin.Coin_C" :Option%201 "/Game/Coin/Coin.Coin_C" :Option%202 "/Game/Coin/Coin.Coin_C" :Option%203 "/Game/Coin/Coin.Coin_C" :Option%204 "/Game/Coin/Coin.Coin_C") (Math|Transform|MakeTransform (Transformation|GetActorLocation) (Math|Rotator|MakeRotator 0.0 0.0 (Math|Random|RandomFloatinRange 0.0 3.6e+02))) "Undefined" 0 0))
  (Utilities|IsValid _returnvalue_2
    (:Is%20Valid
      (Default|RandomMake _returnvalue_2))))

(event EventBeginPlay
  (Utilities|FlowControl|Sequence
    (:then_0
      ;[1 1 1] AI
      (CallFunction|GetEnemy))
    (:then_1
      (CallFunction|BaseMovement))
    (:then_2
      (bind _asai_controller_enemy_bp (Utilities|Casting|CastToAI_Controller_Enemy_BP (Pawn|GetController)))
      (Variables|Default|SetAIController _asai_controller_enemy_bp)
      (AI|SetFocus (Variables|Default|GetAIController) (Variables|Default|GetMy%20Enemy)))
    (:then_3
      ;[1 1 1] 무기 액터 장착
      (bind _returnvalue (Game|SpawnActorfromClass "/Game/Monster/AI/Enemy_Weapon.Enemy_Weapon_C" (Math|Transform|MakeTransform "0, 0, 0") "Undefined" 0 0))
      (bind _output_get (Variables|Default|SetEnemy_Weapon _returnvalue))
      (Transformation|AttachComponentToComponent _output_get (Variables|Character|GetMesh) "SwordSocket" "SnapToTarget" "SnapToTarget" "SnapToTarget" true))))

(fn ConstructionScript)

(fn GetDamage
  (params (DamageSize :type Float%20%28single-precision%29))
  (Variables|Default|SetHealth (- (Variables|Default|GetHealth) DamageSize))
  (Variables|Default|SetstiffSize 1e+02)
  (if (<= (Variables|Default|GetHealth) 0.0)
    (CallFunction|Die)))