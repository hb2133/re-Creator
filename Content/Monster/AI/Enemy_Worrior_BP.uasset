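; Warrior enemy AI Blueprint that arms itself with a spawned weapon on the SwordSocket and melees its MyEnemy target.
; AttackRange overlaps toggle CanAttack and start a looping attack montage, which repeats immediately while alive and undamaged, otherwise after a short delay if still in range.
; The right sword collision damages the target when CanHitR is set, then clears that flag to prevent repeat hits.
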(event OnComponentBeginOverlap(AttackRange)
  (params (OverlappedComponent :type Primitive%20Component%20Object%20Reference) (OtherActor :type Actor%20Object%20Reference) (OtherComp :type Primitive%20Component%20Object%20Reference) (OtherBodyIndex :type Integer) (bFromSweep :type Boolean) (SweepResult :type Hit%20Result%20Structure%20%28by%20ref%29))
  ;[1 1 1] AI
  (if (and (== OtherActor (Variables|Default|GetMy%20Enemy)) (not (Variables|Default|GetIsAttacking)))
    (Variables|Default|SetCanAttack true :!label _label)
    (Variables|Default|SetIsAttacking true :!label _label_2)
    (Animation|Montage|PlayMontage (Variables|Character|GetMesh) "/Game/Monster/AI/Corpse_Alert_Attack_Fast2_Montage.Corpse_Alert_Attack_Fast2_Montage"
      (:OnCompleted
        _)
      (:OnInterrupted
        _))
    (Variables|Default|SetIsAttacking false)
    (if (Math|Boolean|ANDBoolean (Variables|Default|GetCanAttack) (Variables|Default|GetIsAlive) (not (Variables|Default|GetisDamaged)))
      (goto _label_2)
      (else
        (Utilities|FlowControl|Delay 0.7)
        (if (stale OnComponentEndOverlap(AttackRange) _output_get)
          (goto _label))))))

(event OnComponentEndOverlap(AttackRange)
  (params (OverlappedComponent :type Primitive%20Component%20Object%20Reference) (OtherActor :type Actor%20Object%20Reference) (OtherComp :type Primitive%20Component%20Object%20Reference) (OtherBodyIndex :type Integer))
  ;[1 1 1] AI
  (if (and (== OtherActor (Variables|Default|GetMy%20Enemy)) (Variables|Default|GetCanAttack))
    (bind _output_get (Variables|Default|SetCanAttack false))))

(event OnComponentBeginOverlap(SwordCollision_R)
  (params (OverlappedComponent :type Primitive%20Component%20Object%20Reference) (OtherActor :type Actor%20Object%20Reference) (OtherComp :type Primitive%20Component%20Object%20Reference) (OtherBodyIndex :type Integer) (bFromSweep :type Boolean) (SweepResult :type Hit%20Result%20Structure%20%28by%20ref%29))
  ;[1 1 1] AI
  (if (and (== OtherActor (Variables|Default|GetMy%20Enemy)) (Variables|Default|GetCanHit_R))
    (Variables|Default|SetCanHit_R false)
    (Default|TakeDamage (Variables|Default|GetMy%20Enemy) 5.0)))

(event Collision|EventActorBeginOverlap
  (params (OtherActor :type Actor%20Object%20Reference)))

(event EventTick
  (params (DeltaSeconds :type Float%20%28single-precision%29)))

(event EventBeginPlay
  (|CallParentFunction)
  (Utilities|FlowControl|Sequence
    (:then_0
      (bind _returnvalue (Game|SpawnActorfromClass "/Game/Monster/AI/Enemy_Weapon.Enemy_Weapon_C" (Math|Transform|MakeTransform "0, 0, 0") "Undefined" 0 0))
      (bind _output_get (Variables|Default|SetEnemy_Weapon _returnvalue))
      (Transformation|AttachComponentToComponent _output_get (Variables|Character|GetMesh) "SwordSocket" "SnapToTarget" "SnapToTarget" "SnapToTarget" true))
    (:then_1
      (Variables|Default|SetDistance 75.0))))

(fn ConstructionScript
  (|CallParentFunction))