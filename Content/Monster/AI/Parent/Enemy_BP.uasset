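; Parent Blueprint for enemy monsters that chase the player and take damage, leaving AttackStart empty.
; A retrying AIMoveTo loop triggers AttackStart on arrival and waits while attacking or damaged.
; Stagger events (경직/경직끝) unpossess the AI, play hit montage, material flash, sound and shake, then respawn the controller.
; GetDamage spawns damage widgets, a timeline drives damage-over-time, and death drops coins before delayed destruction.
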(event Custom|GetEnemy
  ;[1 1 1] AI
  (Utilities|FlowControl|Delay 1.0)
  (bind _outactors (Actor|GetAllActorsOfClass "/Game/ThirdPersonCPP/Blueprints/ThirdPersonCharacter.ThirdPersonCharacter_C"))
  (Variables|Default|SetMy%20Enemy (Utilities|Array|Get(acopy) _outactors)))

(event Custom|BaseMovement
  ;[1 1 1] AI
  (Utilities|IsValid (Variables|Default|GetMy%20Enemy) :!label _label
    (:Is%20Valid
      (if (Variables|Default|GetIsAlive)
        (if (or (Variables|Default|GetisDamaged) (Variables|Default|GetIsAttacking))
          ;;[1 1 1] 공격후 정지시간
          (Utilities|FlowControl|Delay 0.1 :!label _label_2)
          (goto _label)
          (else
            (AI|AIMoveTo self "0, 0, 0" (Variables|Default|GetMy%20Enemy) (Variables|Default|GetDistance) false
              (:then
                (Variables|Default|SetisMoving true))
              (:OnSuccess
                (Variables|Default|SetisMoving false)
                (CallFunction|AttackStart)
                (goto _label_2))
              (:OnFail
                (goto _label)))))))
    (:Is%20Not%20Valid
      ;;[1 1 1] Nav시작시간
      (Utilities|FlowControl|Delay 0.1)
      (goto _label))))

(event Custom|TakeDamage
  (params (Amount :type Float%20%28single-precision%29))
  (bind _output_get (Variables|Default|SetHealth (- (Variables|Default|GetHealth) Amount)))
  (if (> _output_get 0.0)
    (Development|PrintString (Utilities|String|ToString(Float) (Variables|Default|GetHealth)) true true "(R=1.000000,G=0.000000,B=0.026892,A=1.000000)")
    (else
      (CallFunction|Die))))

(event Custom|Die
  (bind _enemy_weapon (Variables|Default|GetEnemy_Weapon))
  (Utilities|FlowControl|Sequence
    (:then_0
      (Variables|Default|SetIsAlive false)
      (Audio|PlaySound2D (Variables|Default|GetEnemyDIeSound) 1.0 1.0 0.0 "/Game/temporary/NewSoundConcurrency.NewSoundConcurrency" 0)
      (Components|Movement|StopMovementImmediately (Variables|Character|GetCharacterMovement))
      (AI|ClearFocus (Variables|Default|GetAIController))
      (for _index (range 3 5)
        (CallFunction|DropLoot))
      (Utilities|FlowControl|Delay (Math|Conversions|ToFloat(Integer) (Math|Random|RandomIntegerinRange 4 6)))
      (Utilities|IsValid _enemy_weapon
        (:Is%20Valid
          (Actor|DestroyActor _enemy_weapon))
        (:Is%20Not%20Valid
          _))
      (Actor|DestroyActor))
    (:then_1
      (Timeline|DotDam Stop
        (:Finished
          (Utilities|FlowControl|DoOnce false) ; enters at Reset
        )
        (:DotEvent
          (CallFunction|GetDamage (stale Custom|DotDamage DotDamage)))))))

(event Custom|StartRagdoll
  (bind _mesh (Variables|Character|GetMesh))
  (Class|SkeletalMeshComponent|SetAllBodiesSimulatePhysics _mesh true)
  (Collision|SetCollisionProfileName _mesh "Ragdoll" true :!class /Script/Engine.PrimitiveComponent)
  (Collision|SetCollisionEnabled (Variables|Collision|GetCapsuleComponent) "NoCollision"))

(event Custom|경직
  (params (DamageSize :type Float%20%28single-precision%29))
  (bind _returnvalue (Pawn|GetController))
  (bind _mesh (Variables|Character|GetMesh))
  (bind _mesh_2 (Variables|Character|GetMesh))
  (Utilities|IsValid _returnvalue
    (:Is%20Valid
      (Pawn|UnPossess _returnvalue))
    (:Is%20Not%20Valid
      _))
  (CallFunction|GetDamage DamageSize)
  (Variables|Default|SetisDamaged true)
  (Components|Movement|StopMovementImmediately (Variables|Character|GetCharacterMovement))
  (Animation|StopAnimMontage 0)
  (Animation|Montage|PlayMontage (Variables|Character|GetMesh) "/Game/Monster/AI/Monster_Damaged.Monster_Damaged" 0.0 0.0 (Utilities|String|StringToName (Utilities|String|ToString(Integer) (Class|KismetMathLibrary|RandomIntegerfromStream 4 (Variables|Default|GetRandomAnimation))))
    (:then
      (Utilities|FlowControl|Sequence
        (:then_0
          (Rendering|Material|SetMaterial _mesh 0 (Variables|Default|GetM_Inst_Hit))
          (Rendering|Material|SetMaterial _mesh 1 (Variables|Default|GetM_Clothes_Hit))
          (Class|MatineeCameraShake|StartMatineeCameraShake (Game|GetPlayerCameraManager 0) "/Game/Camera/Shake.Shake_C" 0.05 "CameraLocal" "0, 0, 0")
          (Audio|PlaySound2D "/Game/Sound/Monster/Worrior/Worrior_hit.Worrior_hit" 1.0 1.0 0.0 "/Game/temporary/NewSoundConcurrency.NewSoundConcurrency" 0))
        (:then_1
          (Utilities|FlowControl|Delay 0.3)
          (Rendering|Material|SetMaterial _mesh_2 0 (Variables|Default|GetM_Inst))
          (Rendering|Material|SetMaterial _mesh_2 1 (Variables|Default|GetM_Clothes)))))))

(event Custom|경직끝
  (Animation|Montage|PlayMontage (Variables|Character|GetMesh) "/Game/Monster/AI/Monster_Damaged.Monster_Damaged" 4.0 0.0 (Variables|Default|Getaction_Name)
    (:OnCompleted
      _)
    (:OnInterrupted
      (Development|PrintString "몽타주 멈춤!")))
  (Variables|Default|SetisDamaged false)
  (Pawn|SpawnDefaultController))

(event Custom|Drop%20Loot
  (bind _returnvalue (Transformation|GetActorLocation))
  ;[1 1 1] 몬스터의 아이템 드랍
  (bind _outhit (Collision|LineTraceByChannel _returnvalue (- _returnvalue "0, 0,200.000000") "TraceTypeQuery1" false (Utilities|Array|MakeArray (Game|GetPlayerCharacter 0)) "None"))
  (bind _returnvalue_2 (Game|SpawnActorfromClass (Utilities|Select :Index (Math|Random|RandomInteger 5) :Option%200 "/Game/Coin/Coin.Coin_C" :Option%201 "/Game/Coin/Coin.Coin_C" :Option%202 "/Game/Coin/Coin.Coin_C" :Option%203 "/Game/Coin/Coin.Coin_C" :Option%204 "/Game/Coin/Coin.Coin_C") (Math|Transform|MakeTransform (Transformation|GetActorLocation) (Math|Rotator|MakeRotator 0.0 0.0 (Math|Random|RandomFloatinRange 0.0 3.6e+02))) "Undefined" 0 0))
  (Utilities|IsValid _returnvalue_2
    (:Is%20Valid
      (bind _output_get (Variables|/Game/Coin/Coin.Coin_C|SetCoinApply _returnvalue_2 (Math|Float|Ceil (Math|Float|Power (Math|Conversions|ToFloat(Integer) (Variables|Default|GetCost)) 1.5))))
      (Development|PrintString (Utilities|String|ToString(Integer) _output_get))
      (Default|RandomMake _returnvalue_2))))

(event Custom|AttackStart
  ;[1 1 1] 무기 액터 장착
)

(event Custom|DotDamage
  (params (DotDamage :type Float%20%28single-precision%29))
  (Utilities|FlowControl|DoOnce false :!label _label
    (:Completed
      (Timeline|DotDam PlayFromStart
        (:Finished
          (goto _label Reset))
        (:DotEvent
          (CallFunction|GetDamage DotDamage))))))

(event EventBeginPlay
  (Utilities|FlowControl|Sequence
    (:then_0
      ;[1 1 1] AI
      (CallFunction|GetEnemy))
    (:then_1
      (CallFunction|BaseMovement))
    (:then_2
      (bind _asai_controller_enemy_bp (Utilities|Casting|CastToAI_Controller_Enemy_BP (Pawn|GetController)))
      (Variables|Default|SetAIController _asai_controller_enemy_bp)
      (AI|SetFocus (Variables|Default|GetAIController) (Variables|Default|GetMy%20Enemy)))
    (:then_3
      (Variables|Default|SetSelfRef self))))

(fn ConstructionScript)

(fn GetDamage
  (params (DamageSize :type Float%20%28single-precision%29))
  (Game|SpawnActorfromClass "/Game/UI/BP_DamageWidget.BP_DamageWidget_C" (Math|Conversions|ToTransform(Vector) (+ (Transformation|GetActorLocation) (Math|Vector|MakeVector (Math|Random|RandomFloatinRange -2e+01 2e+01) 7e+01 (Math|Random|RandomFloatinRange 175.0 225.0)))) "Undefined" 0 DamageSize 0)
  (Variables|Default|SetHealth (- (Variables|Default|GetHealth) DamageSize))
  (Variables|Default|SetstiffSize 1e+02)
  (if (<= (Variables|Default|GetHealth) 0.0)
    (CallFunction|Die)))

(fn MoveAI)