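; Assassin enemy Blueprint: a suicide bomber that rushes at high speed, then explodes and dies.
; AttackStart raises speed and starts a looping sound and material blink.
; HitRange overlap unpossesses it, halts movement and plays a faster-flashing, super-armored windup montage before spawning BoomRange, effects and decal.
; Without super armor, 경직 applies damage with a frozen random hit pose, material flash and camera shake; 경직끝 plays out the recovery.
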(event OnComponentBeginOverlap(HitRange)
  (params (OverlappedComponent :type Primitive%20Component%20Object%20Reference) (OtherActor :type Actor%20Object%20Reference) (OtherComp :type Primitive%20Component%20Object%20Reference) (OtherBodyIndex :type Integer) (bFromSweep :type Boolean) (SweepResult :type Hit%20Result%20Structure%20%28by%20ref%29))
  (bind _returnvalue (Pawn|GetController))
  (bind _returnvalue_2 (Transformation|GetActorTransform))
  (bind _returnvalue_3 (Transformation|GetActorTransform))
  (Utilities|FlowControl|DoOnce false
    (:Completed
      (Utilities|IsValid _returnvalue
        (:Is%20Valid
          (Pawn|UnPossess _returnvalue))
        (:Is%20Not%20Valid
          _))
      (Variables|Default|SetIsAttacking true)
      (Pawn|Components|CharacterMovement|SetMovementMode (Variables|Character|GetCharacterMovement) "MOVE_None" 0)
      (Utilities|Time|ClearandInvalidateTimerbyHandle (stale EventAttackStart _returnvalue_2))
      (bind _returnvalue_4 (Utilities|Time|SetTimerbyEvent (delegate Custom|FinishSkill) 0.1 true))
      (Animation|Montage|PlayMontage (Variables|Character|GetMesh) "/Game/Monster/AI/Assassin/Crouching_Idle_Montage.Crouching_Idle_Montage" 2.5
        (:then
          (Variables|Default|SetSuperArmor true)
          (Components|Activation|SetActive (stale EventAttackStart _returnvalue) false false))
        (:OnCompleted
          (Effects|SpawnEmitteratLocation "/Game/StarterContent/Particles/P_Explosion.P_Explosion" (.location _returnvalue_3) (.rotation _returnvalue_3) "10.000000,10.000000,10.000000")
          (Utilities|Time|ClearandInvalidateTimerbyHandle _returnvalue_4)
          (Rendering|Material|SetMaterial (Variables|Character|GetMesh) 1 "/Game/CityofBrass_Enemies/Materials/Sploder_Inst.Sploder_Inst")
          (Rendering|Material|SetMaterial (Variables|Character|GetMesh) 0 "/Game/CityofBrass_Enemies/Materials/SploderBody_Inst1.SploderBody_Inst1")
          (Game|SpawnActorfromClass "/Game/Monster/AI/Assassin/BoomRange.BoomRange_C" (Math|Transform|MakeTransform (.location _returnvalue_2) (.rotation _returnvalue_2) "6.000000,6.000000,3.000000") "Undefined" 0 0)
          (Game|SpawnActorfromClass "/Game/Effect/Bang/ExplosionDecal_BP.ExplosionDecal_BP_C" (Math|Transform|MakeTransform (+ (.location _returnvalue_2) (* (Transformation|GetActorUpVector) -5.0)) "90.000000, 0, 0" "1,1,1") "Undefined" 0 0)
          (Audio|PlaySound2D "/Game/Sound/Monster/assassin/explosion.explosion" 1.0 1.0 0.0 0 0)
          (CallFunction|Die))))))

(event Custom|Explosionable
  (bind _mesh (Variables|Character|GetMesh))
  (Utilities|FlowControl|FlipFlop
    (:A
      (Rendering|Material|SetMaterial _mesh 1 "/Game/Monster/AI/Assassin/Sploder_Inst1.Sploder_Inst1"))
    (:B
      (Rendering|Material|SetMaterial _mesh 1 "/Game/CityofBrass_Enemies/Materials/Sploder_Inst.Sploder_Inst"))))

(event Custom|FinishSkill
  (Utilities|FlowControl|FlipFlop
    (:A
      (Rendering|Material|SetMaterial (Variables|Character|GetMesh) 1 "/Game/Monster/AI/Assassin/Sploder_Inst1.Sploder_Inst1")
      (Rendering|Material|SetMaterial (Variables|Character|GetMesh) 0 "/Game/Monster/AI/Assassin/SploderBody_Inst2.SploderBody_Inst2"))
    (:B
      (Rendering|Material|SetMaterial (Variables|Character|GetMesh) 1 "/Game/CityofBrass_Enemies/Materials/Sploder_Inst.Sploder_Inst")
      (Rendering|Material|SetMaterial (Variables|Character|GetMesh) 0 "/Game/CityofBrass_Enemies/Materials/SploderBody_Inst1.SploderBody_Inst1"))))

(event EventBeginPlay
  (|CallParentFunction)
  (Utilities|FlowControl|Sequence
    (:then_0
      (Variables|Default|SetDistance 8e+02))
    (:then_1
      (Variables|Default|SetM_Inst "/Game/CityofBrass_Enemies/Materials/SploderBody_Inst1.SploderBody_Inst1")
      (Variables|Default|SetM_Clothes "/Game/CityofBrass_Enemies/Materials/Sploder_Inst.Sploder_Inst"))
    (:then_2
      (Variables|/Script/Engine.CharacterMovementComponent|SetMaxWalkSpeed (Variables|Character|GetCharacterMovement) 1e+02))
    (:then_3
      (Variables|Default|SetEnemyDIeSound "/Game/Sound/Monster/Worrior/Worrior_dead.Worrior_dead"))))

(event Collision|EventActorBeginOverlap
  (params (OtherActor :type Actor%20Object%20Reference)))

(event EventAttackStart
  (Utilities|FlowControl|DoOnce false
    (:Completed
      (Variables|Default|SetIsAttacking false)
      (Variables|Default|SetDistance 5e+01)
      (Variables|/Script/Engine.CharacterMovementComponent|SetMaxWalkSpeed (Variables|Character|GetCharacterMovement) 9e+02)
      (bind _returnvalue (Audio|SpawnSound2D "/Game/Sound/Monster/assassin/skull해골턱소리.skull해골턱소리" 1.0 1.0 0.0 0))
      (bind _returnvalue_2 (Utilities|Time|SetTimerbyEvent (delegate Custom|Explosionable) 0.7 true)))))

(event Event경직
  (params (DamageSize :type Float%20%28single-precision%29))
  (bind _mesh (Variables|Character|GetMesh))
  (bind _mesh_2 (Variables|Character|GetMesh))
  (if (not (Variables|Default|GetSuperArmor))
    (CallFunction|GetDamage DamageSize)
    (Variables|Default|SetisDamaged true)
    (Components|Movement|StopMovementImmediately (Variables|Character|GetCharacterMovement))
    (Animation|Montage|PlayMontage (Variables|Character|GetMesh) "/Game/Monster/AI/Monster_Damaged.Monster_Damaged" 0.0 0.0 (Utilities|String|StringToName (Utilities|String|ToString(Integer) (Class|KismetMathLibrary|RandomIntegerfromStream 4 (Variables|Default|GetRandomAnimation))))
      (:then
        (Utilities|FlowControl|Sequence
          (:then_0
            (Rendering|Material|SetMaterial _mesh 0 (Variables|Default|GetM_Inst_Hit))
            (Rendering|Material|SetMaterial _mesh 1 (Variables|Default|GetM_Clothes_Hit))
            (Class|MatineeCameraShake|StartMatineeCameraShake (Game|GetPlayerCameraManager 0) "/Game/Camera/Shake.Shake_C" 0.05 "CameraLocal" "0, 0, 0")
            (Audio|PlaySound2D "/Game/Sound/Monster/Worrior/Worrior_hit.Worrior_hit" 1.0 1.0 0.0 "/Game/temporary/NewSoundConcurrency.NewSoundConcurrency" 0))
          (:then_1
            (Utilities|FlowControl|Delay 0.3)
            (Rendering|Material|SetMaterial _mesh_2 0 (Variables|Default|GetM_Inst))
            (Rendering|Material|SetMaterial _mesh_2 1 (Variables|Default|GetM_Clothes))))))))

(event Event경직끝
  (if (not (Variables|Default|GetSuperArmor))
    (Animation|Montage|PlayMontage (Variables|Character|GetMesh) "/Game/Monster/AI/Monster_Damaged.Monster_Damaged" 4.0 0.0 "action"
      (:OnCompleted
        _)
      (:OnInterrupted
        (Development|PrintString "몽타주 멈춤!")))
    (Variables|Default|SetisDamaged false)))

(fn ConstructionScript
  (|CallParentFunction))