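; Magician enemy AI that chases its target to casting range and drops fire fields on it.
; ReSkill marks the target's position with a fire effect and starts a timer; Skill then plays the cast montage, whose notify replaces the effect with a scaled-up FireField before movement resumes.
; Taking damage freezes a random hit pose with material flash, camera shake and sound, cancels the timer, and restarts any pending cast after a delay.
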(event Custom|Skill
  (if true
    _
    (else
      _))
  (Utilities|IsValid (Variables|Default|GetMy%20Enemy)
    (:Is%20Valid
      (if (not (Variables|Default|GetisMoving))
        (Utilities|Time|ClearandInvalidateTimerbyHandle (Variables|Default|GetSkillTimer))
        (Animation|Montage|PlayMontage (Variables|Character|GetMesh) "/Game/Monster/AI/Magician/Standing_2H_Cast_Spell_01_Montage.Standing_2H_Cast_Spell_01_Montage"
          (:OnCompleted
            (CallFunction|BaseMovement :!label _label))
          (:OnInterrupted
            (goto _label))
          (:OnNotifyBegin
            (Utilities|FlowControl|Sequence
              (:then_0
                (Utilities|IsValid (stale Custom|ReSkill _returnvalue_3)
                  (:Is%20Valid
                    (Game|SpawnActorfromClass "/Game/Monster/AI/Magician/FireField.FireField_C" (Math|Transform|MakeTransform (.location (Transformation|GetActorTransform (stale Custom|ReSkill _returnvalue_3))) (.rotation (Transformation|GetActorTransform (stale Custom|ReSkill _returnvalue_3))) "10.000000,10.000000,10.000000") "Undefined" 0 0)
                    (Actor|DestroyActor (stale Custom|ReSkill _returnvalue_3))))))))))))

(event Custom|ReSkill
  (bind _returnvalue (Transformation|GetActorLocation))
  (bind _returnvalue_2 (Utilities|Time|SetTimerbyEvent (delegate Custom|Skill) 3.0 true))
  (Variables|Default|SetSkillTimer _returnvalue_2)
  (Transformation|SetActorLocationAndRotation _returnvalue (Math|Rotator|FindLookatRotation _returnvalue (Transformation|GetActorLocation (Variables|Default|GetMy%20Enemy))))
  (bind _returnvalue_3 (Game|SpawnActorfromClass "/Game/StarterContent/Blueprints/Blueprint_Effect_Fire.Blueprint_Effect_Fire_C" (Transformation|GetActorTransform (Variables|Default|GetMy%20Enemy)) "Undefined" 0 0)))

(event Event경직
  (params (DamageSize :type Float%20%28single-precision%29))
  (bind _mesh (Variables|Character|GetMesh))
  (bind _mesh_2 (Variables|Character|GetMesh))
  (CallFunction|GetDamage DamageSize)
  (Variables|Default|SetisDamaged true)
  (Components|Movement|StopMovementImmediately (Variables|Character|GetCharacterMovement))
  (Animation|Montage|PlayMontage (Variables|Character|GetMesh) "/Game/Monster/AI/Monster_Damaged.Monster_Damaged" 0.0 0.0 (Utilities|String|StringToName (Utilities|String|ToString(Integer) (Class|KismetMathLibrary|RandomIntegerfromStream 4 (Variables|Default|GetRandomAnimation))))
    (:then
      (Utilities|FlowControl|Sequence
        (:then_0
          (Rendering|Material|SetMaterial _mesh_2 0 (Variables|Default|GetM_Inst_Hit))
          (Rendering|Material|SetMaterial _mesh_2 1 (Variables|Default|GetM_Clothes_Hit))
          (Class|MatineeCameraShake|StartMatineeCameraShake (Game|GetPlayerCameraManager 0) "/Game/Camera/Shake.Shake_C" 0.05 "CameraLocal" "0, 0, 0")
          (Audio|PlaySound2D 0 1.0 1.0 0.0 0 0)
          (Audio|PlaySound2D 0 1.0 1.0 0.0 0 0))
        (:then_1
          (Utilities|FlowControl|Delay 0.3)
          (Rendering|Material|SetMaterial _mesh 0 "/Game/CityofBrass_Enemies/Materials/Wizard_Inst.Wizard_Inst")
          (Rendering|Material|SetMaterial _mesh 1 "/Game/CityofBrass_Enemies/Materials/FermaleWarrior_Inst.FermaleWarrior_Inst"))
        (:then_2
          (Utilities|Time|ClearandInvalidateTimerbyHandle (Variables|Default|GetSkillTimer))
          (Utilities|IsValid (stale Custom|ReSkill _returnvalue_3)
            (:Is%20Valid
              (Actor|DestroyActor (stale Custom|ReSkill _returnvalue_3))
              (Utilities|FlowControl|Delay 0.5)
              (CallFunction|ReSkill))))))))

(event Collision|EventActorBeginOverlap
  (params (OtherActor :type Actor%20Object%20Reference)))

(event Event경직끝
  (Animation|Montage|PlayMontage (Variables|Character|GetMesh) "/Game/Monster/AI/Monster_Damaged.Monster_Damaged" 4.0 0.0 "action"
    (:OnCompleted
      _)
    (:OnInterrupted
      (Development|PrintString "몽타주 멈춤!")))
  (Variables|Default|SetisDamaged false))

(event EventTick
  (params (DeltaSeconds :type Float%20%28single-precision%29))
  (Utilities|FlowControl|Sequence
    (:then_0
      (Transformation|AddLocalRotation (Variables|Default|GetPoseableMesh) "2.000000, 0, 0" false false)
      (Development|PrintString (Utilities|String|ToString(Float) (Utilities|Time|GetTimerRemainingTimebyHandle (Variables|Default|GetSkillTimer)))))))

(event EventBeginPlay
  (|CallParentFunction)
  (Utilities|FlowControl|Sequence
    (:then_1
      (Variables|Default|SetDistance 5e+02))
    (:then_2
      (Variables|Default|SetM_Inst "/Game/CityofBrass_Enemies/Materials/Corpse_Body_Inst2.Corpse_Body_Inst2")
      (Variables|Default|SetM_Clothes "/Game/CityofBrass_Enemies/Materials/Corpse_Clothes_Inst.Corpse_Clothes_Inst"))))

(event EventBaseMovement
  (bind _returnvalue (Transformation|GetActorLocation))
  (Utilities|IsValid (Variables|Default|GetMy%20Enemy) :!label _label
    (:Is%20Valid
      (if (Variables|Default|GetIsAlive)
        (if (not (Variables|Default|GetIsAttacking))
          (AI|AIMoveTo self "0, 0, 0" (Variables|Default|GetMy%20Enemy) (Variables|Default|GetDistance) false
            (:then
              (Variables|Default|SetisMoving true))
            (:OnSuccess
              (Variables|Default|SetisMoving false)
              (bind _returnvalue_2 (Utilities|Time|SetTimerbyEvent (delegate Custom|Skill) 3.0 true))
              (Variables|Default|SetSkillTimer _returnvalue_2)
              (Transformation|SetActorLocationAndRotation _returnvalue (Math|Rotator|FindLookatRotation _returnvalue (Transformation|GetActorLocation (Variables|Default|GetMy%20Enemy))))
              (bind _returnvalue_3 (Game|SpawnActorfromClass "/Game/StarterContent/Blueprints/Blueprint_Effect_Fire.Blueprint_Effect_Fire_C" (Transformation|GetActorTransform (Variables|Default|GetMy%20Enemy)) "Undefined" 0 0)))
            (:OnFail
              (goto _label))))))
    (:Is%20Not%20Valid
      ;[1 1 1] Nav시작시간
      (Utilities|FlowControl|Delay 0.1)
      (goto _label))))

(fn ConstructionScript
  (|CallParentFunction))