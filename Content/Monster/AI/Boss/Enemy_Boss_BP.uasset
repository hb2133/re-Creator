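; Boss enemy that chases the player with AI MoveTo, makes melee attacks on overlap and fires skills on a cooldown timeline.
; Above a health threshold it picks one of six montage skills, using notifies to time telegraphs and hits.
; Below it, a hardwired branch moves it to a fixed point to send out five ghosts.
; Hits flash materials and update the HP widget; death triggers ragdoll, ending widgets and the end level.
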(event OnComponentBeginOverlap(SwordCollision_R)
  (params (OverlappedComponent :type Primitive%20Component%20Object%20Reference) (OtherActor :type Actor%20Object%20Reference) (OtherComp :type Primitive%20Component%20Object%20Reference) (OtherBodyIndex :type Integer) (bFromSweep :type Boolean) (SweepResult :type Hit%20Result%20Structure%20%28by%20ref%29))
  ;[1 1 1] 기본 공격
  (if (== OtherActor (Variables|Default|GetMy%20Enemy))
    (Variables|Default|SetCanHit_R false)
    (Development|PrintString "오른손")
    (Default|TakeDamage (Variables|Default|GetMy%20Enemy) 1.0)
    (Collision|SetCollisionEnabled (Variables|Default|GetSwordCollision_R) "NoCollision")))

(event OnComponentBeginOverlap(AttackRange)
  (params (OverlappedComponent :type Primitive%20Component%20Object%20Reference) (OtherActor :type Actor%20Object%20Reference) (OtherComp :type Primitive%20Component%20Object%20Reference) (OtherBodyIndex :type Integer) (bFromSweep :type Boolean) (SweepResult :type Hit%20Result%20Structure%20%28by%20ref%29))
  (bind _returnvalue (Pawn|GetController))
  ;[1 1 1] 기본 공격
  (if (and (== OtherActor (Variables|Default|GetMy%20Enemy)) (not (Variables|Default|GetIsAttacking)))
    (Variables|Default|SetIsAttacking true)
    (Collision|SetCollisionEnabled (Variables|Default|GetAttackRange) "NoCollision")
    (Transformation|SetActorRotation (Math|Conversions|RotationFromXVector (- (Transformation|GetActorLocation (Variables|Default|GetMy%20Enemy)) (Transformation|GetActorLocation))))
    (Utilities|IsValid _returnvalue
      (:Is%20Valid
        (Pawn|UnPossess _returnvalue))
      (:Is%20Not%20Valid
        _))
    (Animation|Montage|PlayMontage (Variables|Character|GetMesh) "/Game/Monster/AI/Boss/SkillType/Attack_Boss.Attack_Boss"
      (:OnCompleted
        (Utilities|FlowControl|Delay 0.2)
        (Variables|Default|SetIsAttacking false)
        (if (Variables|Default|GetIsSkill)
          (CallFunction|SkillStart)
          (elif (< (Math|Vector|Distance(Vector) (Transformation|GetActorLocation (Variables|Default|GetMy%20Enemy)) (Transformation|GetActorLocation)) 2e+02)
            (Collision|SetCollisionEnabled (Variables|Default|GetAttackRange) "QueryOnly")
            (else
              (CallFunction|Chase))))))))

(event OnComponentBeginOverlap(SwordCollision_L)
  (params (OverlappedComponent :type Primitive%20Component%20Object%20Reference) (OtherActor :type Actor%20Object%20Reference) (OtherComp :type Primitive%20Component%20Object%20Reference) (OtherBodyIndex :type Integer) (bFromSweep :type Boolean) (SweepResult :type Hit%20Result%20Structure%20%28by%20ref%29))
  ;[1 1 1] 기본 공격
  (if (== OtherActor (Variables|Default|GetMy%20Enemy))
    (Variables|Default|SetCanHit_L false)
    (Development|PrintString "왼손")
    (Default|TakeDamage (Variables|Default|GetMy%20Enemy) 1.0)
    (Collision|SetCollisionEnabled (Variables|Default|GetSwordCollision_L) "NoCollision")))

(event OnComponentBeginOverlap(SkillBody)
  (params (OverlappedComponent :type Primitive%20Component%20Object%20Reference) (OtherActor :type Actor%20Object%20Reference) (OtherComp :type Primitive%20Component%20Object%20Reference) (OtherBodyIndex :type Integer) (bFromSweep :type Boolean) (SweepResult :type Hit%20Result%20Structure%20%28by%20ref%29))
  (bind _mesh (Variables|Character|GetMesh))
  (bind _my_enemy (Variables|Default|GetMy%20Enemy))
  (bind _returnvalue (Transformation|GetActorTransform _my_enemy))
  (bind _returnvalue_2 (Components|SkeletalMesh|GetAnimInstance _mesh))
  (Development|PrintString "충돌!!!!!!!!!!!!!!!!1!")
  (if (== OtherActor (Variables|Default|GetMy%20Enemy))
    (switch name (Animation|Montage|MontageGetCurrentSection _returnvalue_2 (Animation|Montage|GetCurrentActiveMontage _returnvalue_2))
      (:Attack
        (Default|TakeDamage (Variables|Default|GetMy%20Enemy) 5e+01))
      (:Dash
        (Transformation|SetActorTransform _my_enemy (Math|Transform|MakeTransform (.location _returnvalue) (Math|Conversions|RotationFromXVector (* (Math|Vector|GetForwardVector (Transformation|GetActorRotation)) -1.0)) (.scale _returnvalue)))
        (Animation|Montage|PlayMontage (Variables|/Script/Engine.Character|GetMesh _my_enemy) "/Game/Player_Taunt_Montage.Player_Taunt_Montage"
          (:then
            (Default|TakeDamage (Variables|Default|GetMy%20Enemy) 3e+01))))
      (:Spin
        (Default|TakeDamage (Variables|Default|GetMy%20Enemy) 5e+01)
        (Transformation|SetRelativeScale3D (Variables|Default|GetSkillBody) "3.000000,3.000000,3.000000")))))

(event Custom|SkillStart
  (bind _returnvalue (Transformation|GetActorTransform))
  (bind _returnvalue_2 (Transformation|GetActorTransform))
  (bind _returnvalue_3 (Transformation|GetActorTransform))
  (bind _returnvalue_4 (Pawn|GetController))
  (bind _self self)
  (bind _health (Variables|Default|GetHealth))
  (bind _returnvalue_5 (> _health 7e+03))
  (if (Math|Boolean|ANDBoolean (not (Variables|Default|GetIsAttacking)) (Variables|Default|GetIsSkill) (Variables|Default|GetIsAlive))
    (if _returnvalue_5
      (Utilities|IsValid _returnvalue_4 :!label _label
        (:Is%20Valid
          (Pawn|UnPossess _returnvalue_4))
        (:Is%20Not%20Valid
          _))
      (for _array_element (Variables|Default|GetCollision)
        (Collision|SetCollisionEnabled _array_element "NoCollision"))
      (Variables|Default|SetSkillRotate (Transformation|GetActorRotation))
      (Utilities|FlowControl|Delay 0.2)
      (Variables|Default|SetIsAttacking true)
      (bind _output_get (Variables|Default|SetSkillInt (Math|Random|RandomIntegerinRange 0 5)))
      (switch int _output_get
        (:0
          ;[1 1 1] 저돌맹진
          (Animation|Montage|PlayMontage (Variables|Character|GetMesh) "/Game/Monster/AI/Boss/SkillType/Dash_Boss.Dash_Boss" 1.2
            (:OnCompleted
              (if _returnvalue_5 :!label _label_2
                _
                (else
                  (Game|SpawnActorfromClass "/Game/Effect/Monster_Effect/Boss_Ghost/Enemy_Boss_Ghost_BP.Enemy_Boss_Ghost_BP_C" (Transformation|GetActorTransform) "Undefined" 0 self)))
              (Collision|SetCollisionEnabled (Variables|Default|GetSkillBody) "NoCollision" :!label _label_3)
              (Transformation|SetRelativeScale3D (Variables|Default|GetSkillBody) "3.000000,3.000000,3.000000")
              (Variables|Default|SetIsAttacking false)
              (Variables|Default|SetIsSkill false)
              (CallFunction|CoolTime)
              (CallFunction|Chase))
            (:OnInterrupted
              (goto _label_2))
            (:OnNotifyBegin
              (bind _returnvalue_6 (Game|SpawnActorfromClass "/Game/Monster/AI/Boss/SkillType/Skill/DashAttack_AOE.DashAttack_AOE_C" (Math|Transform|MakeTransform (+ (* (Transformation|GetActorForwardVector) 2e+02) (.location _returnvalue_3)) (.rotation _returnvalue_3) "1,1,1") "Undefined" 0 self)))
            (:OnNotifyEnd
              (Collision|SetCollisionEnabled (Variables|Default|GetSkillBody) "QueryOnly")
              (Actor|DestroyActor _returnvalue_6))))
        (:1
          ;[1 1 1] 탈태
          (Variables|Default|SetplayerTransform (Transformation|GetActorTransform (Variables|Default|GetMy%20Enemy)))
          (Transformation|SetRelativeScale3D (Variables|Default|GetSkillBody) "9.000000,9.000000,9.000000")
          (Animation|Montage|PlayMontage (Variables|Character|GetMesh) "/Game/Monster/AI/Boss/SkillType/Spin_Boss.Spin_Boss" 1.2
            (:OnCompleted
              (goto _label_2))
            (:OnInterrupted
              (goto _label_2))
            (:OnNotifyBegin
              (bind _returnvalue_7 (Game|SpawnActorfromClass "/Game/Monster/AI/Boss/SkillType/Skill/SpinAttack_AOE.SpinAttack_AOE_C" (Variables|Default|GetplayerTransform) "Undefined" 0 0)))
            (:OnNotifyEnd
              (Collision|SetCollisionEnabled (Variables|Default|GetSkillBody) "QueryOnly")
              (Transformation|SetActorLocationAndRotation (.Location (Math|Transform|BreakTransform (Variables|Default|GetplayerTransform))) (Transformation|GetActorRotation))
              (Actor|DestroyActor _returnvalue_7))))
        (:2
          ;[1 1 1] 천둥호출
          (Animation|Montage|PlayMontage (Variables|Character|GetMesh) "/Game/Monster/AI/Boss/Boss_Cast_Montage.Boss_Cast_Montage" 1.2
            (:OnCompleted
              (goto _label_2))
            (:OnInterrupted
              (goto _label_2))
            (:OnNotifyBegin
              (Timeline|ThunderCycle PlayFromStart
                (:Thunder
                  (bind _output_get_2 (Variables|Default|SetplayerTransform (Transformation|GetActorTransform (Variables|Default|GetMy%20Enemy))))
                  (Game|SpawnActorfromClass "/Game/Monster/AI/Boss/SkillType/Skill/ThunderAttack_AOE.ThunderAttack_AOE_C" _output_get_2 "Undefined" 0 0))))))
        (:3
          ;[1 1 1] 일섬
          (Animation|Montage|PlayMontage (Variables|Character|GetMesh) "/Game/Monster/AI/Boss/SkillType/Cast_Montage.Cast_Montage" 1.2
            (:OnCompleted
              (goto _label_2))
            (:OnInterrupted
              (goto _label_2))
            (:OnNotifyBegin
              (bind _returnvalue_8 (Game|SpawnActorfromClass "/Game/Monster/AI/Boss/SkillType/Skill/RailAttack_AOE.RailAttack_AOE_C" (Math|Transform|MakeTransform (+ (* (Transformation|GetActorForwardVector) 2e+02) (.location _returnvalue)) (.rotation _returnvalue) "1,1,1") "Undefined" 0 self)))
            (:OnNotifyEnd
              (Game|SpawnActorfromClass "/Game/Monster/AI/Boss/SkillType/Skill/RailAttack.RailAttack_C" (Math|Transform|MakeTransform (+ (* (Math|Vector|GetForwardVector (Variables|/Game/Monster/AI/Boss/SkillType/Skill/RailAttack_AOE.RailAttack_AOE_C|GetPlane _returnvalue_8)) -8e+02) (.location (Transformation|GetActorTransform _returnvalue_8))) (.rotation (Transformation|GetActorTransform _returnvalue_8)) "1,1,1") "Undefined" 0 0)
              (Actor|DestroyActor _returnvalue_8))))
        (:4
          ;[1 1 1] 방전
          (Animation|Montage|PlayMontage (Variables|Character|GetMesh) "/Game/Monster/AI/Boss/Standing_Taunt_Battlecry_Montage.Standing_Taunt_Battlecry_Montage" 1.2
            (:OnCompleted
              (goto _label_2))
            (:OnInterrupted
              (goto _label_2))
            (:OnNotifyBegin
              (bind _returnvalue_9 (Game|SpawnActorfromClass "/Game/Monster/AI/Boss/SkillType/Skill/AroundAttack_AOE.AroundAttack_AOE_C" (Math|Transform|MakeTransform (.location _returnvalue_2) (.rotation _returnvalue_2) "10.000000,10.000000,10.000000") "Undefined" 0 0)))
            (:OnNotifyEnd
              (Game|SpawnActorfromClass "/Game/Monster/AI/Boss/SkillType/Skill/AroundAttack.AroundAttack_C" (Math|Transform|MakeTransform (.location _returnvalue_2) (.rotation _returnvalue_2) "10.000000,10.000000,10.000000") "Undefined" 0 0)
              (Actor|DestroyActor _returnvalue_9))))
        (:5
          ;[1 1 1] 휩쓸기
          (Variables|Default|SetMyTransform (Transformation|GetActorTransform))
          (Animation|Montage|PlayMontage (Variables|Character|GetMesh) "/Game/Monster/AI/Boss/SkillType/Brush_Boss.Brush_Boss" 1.2
            (:OnCompleted
              (goto _label_2))
            (:OnInterrupted
              (goto _label_2))
            (:OnNotifyBegin
              (bind _returnvalue_10 (Game|SpawnActorfromClass "/Game/Monster/AI/Boss/SkillType/Skill/PizzaAttack_AOE.PizzaAttack_AOE_C" (Math|Transform|MakeTransform (.location _returnvalue_2) (Math|Rotator|MakeRotator 0.0 0.0 (+ (.Yaw (Math|Rotator|BreakRotator (.rotation _returnvalue_2))) 1.8e+02)) "10.000000,10.000000,1") "Undefined" 0 0)))
            (:OnNotifyEnd
              (Game|SpawnActorfromClass "/Game/Monster/AI/Boss/SkillType/Skill/PizzaAttack_R.PizzaAttack_R_C" (Math|Transform|MakeTransform (.location (Variables|Default|GetMyTransform)) (.rotation (Variables|Default|GetMyTransform)) "2.000000,1.000000,1.000000") "Undefined" 0 _self)
              (Game|SpawnActorfromClass "/Game/Monster/AI/Boss/SkillType/Skill/PizzaAttack_L.PizzaAttack_L_C" (Math|Transform|MakeTransform (.location (Variables|Default|GetMyTransform)) (.rotation (Variables|Default|GetMyTransform)) "2.000000,1.000000,1") "Undefined" 0 _self)
              (Actor|DestroyActor _returnvalue_10)))))
      (else
        (Utilities|FlowControl|Sequence
          (:then_1
            (switch int 2
              (:0
                (Variables|Default|SetPhase2GhostSkill 1)
                (goto _label))
              (:1
                (Pawn|SpawnDefaultController)
                (AI|AIMoveTo self (Math|Vector|MakeVector 4e+02 8e+02 (.z (Transformation|GetActorLocation))) 0 5.0 false
                  (:OnSuccess
                    (Variables|Default|SetPhase2GhostSkill 0)
                    (goto _label_2))))
              (:2
                (Pawn|SpawnDefaultController)
                (AI|AIMoveTo self (Math|Vector|MakeVector 4e+02 8e+02 (.z (Transformation|GetActorLocation))) 0 5.0 false
                  (:OnSuccess
                    (Variables|Default|SetPhase2GhostSkill 2)
                    (for _array_element_2 (Utilities|Array|MakeArray "600.000000,-660.000000,378.019043" "1400.000000,-400.000000,378.019043" "1800.000000,800.000000,378.019043" "1400.000000,1800.000000,378.019043" "600.000000,2100.000000,378.019043")
                      (bind _returnvalue_11 (Game|SpawnActorfromClass "/Game/Effect/Monster_Effect/Boss_Ghost/Enemy_Boss_Ghost_BP.Enemy_Boss_Ghost_BP_C" (Transformation|GetActorTransform) "Undefined" 0 self))
                      (AI|AIMoveTo _returnvalue_11 _array_element_2 0 5.0 false))
                    (goto _label_3)))))))))))

(event Custom|Chase
  (if (Variables|Default|GetIsAlive)
    (Pawn|SpawnDefaultController)
    (Utilities|IsValid (Variables|Default|GetMy%20Enemy)
      (:Is%20Valid
        (Collision|SetCollisionEnabled (Variables|Default|GetAttackRange) "QueryOnly")
        (bind _movementresult (AI|AIMoveTo self "0, 0, 0" (Variables|Default|GetMy%20Enemy) (Variables|Default|GetDistance) false)))
      (:Is%20Not%20Valid
        (Development|PrintString "누구 쫒아가야되;;")))))

(event Custom|CoolTime
  (Timeline|Cool_Time PlayFromStart
    (:Finished
      (Variables|Default|SetIsSkill true)
      (CallFunction|SkillStart))))

(event EventBeginPlay
  (Utilities|FlowControl|Sequence
    (:then_0
      (|CallParentFunction)
      (Variables|/Script/Engine.CharacterMovementComponent|SetMaxWalkSpeed (Variables|Character|GetCharacterMovement) 3e+02)
      (Utilities|FlowControl|Sequence
        (:then_0
          (Variables|Default|SetDistance 8e+01))
        (:then_1
          (Variables|Default|SetM_Inst "/Game/CityofBrass_Enemies/Materials/Corpse_Body_Inst2.Corpse_Body_Inst2")
          (Variables|Default|SetM_Clothes "/Game/CityofBrass_Enemies/Materials/Corpse_Clothes_Inst.Corpse_Clothes_Inst"))
        (:then_2
          (Variables|Default|SetHealth 1e+04))))
    (:then_1
      (bind _returnvalue (UserInterface|CreateWidget "/Game/UI/Boss_HP.Boss_HP_C"))
      (bind _output_get (Variables|Default|SetBoss_HPWidget _returnvalue))
      (UserInterface|Viewport|AddtoViewport _output_get 0))
    (:then_2
      (CallFunction|콜리전비활성화))))

(event Collision|EventActorBeginOverlap
  (params (OtherActor :type Actor%20Object%20Reference)))

(event Event경직
  (params (DamageSize :type Float%20%28single-precision%29))
  (bind _mesh (Variables|Character|GetMesh))
  ;[1 1 1] 경직
  (Variables|/Game/UI/Boss_HP.Boss_HP_C|SetBoss_Health (Variables|Default|GetBoss_HPWidget) (- (Variables|/Game/UI/Boss_HP.Boss_HP_C|GetBoss_Health (Variables|Default|GetBoss_HPWidget)) DamageSize))
  (CallFunction|GetDamage DamageSize)
  (Utilities|FlowControl|Sequence
    (:then_0
      (Rendering|Material|SetMaterial _mesh 0 (Variables|Default|GetM_Inst_Hit))
      (Rendering|Material|SetMaterial _mesh 1 (Variables|Default|GetM_Clothes_Hit)))
    (:then_1
      (Utilities|FlowControl|Delay 0.3)
      (Rendering|Material|SetMaterial _mesh 0 "/Game/CityofBrass_Enemies/Materials/Hooker_Inst.Hooker_Inst")
      (Rendering|Material|SetMaterial _mesh 1 "/Game/CityofBrass_Enemies/Materials/Large_Inst.Large_Inst"))
    (:then_2
      (if (not (> (Variables|/Game/UI/Boss_HP.Boss_HP_C|GetBoss_Health (Variables|Default|GetBoss_HPWidget)) 0.0))
        (CallFunction|Die)
        (Default|WidgetBossHealth (Variables|Default|GetBoss_HPWidget))
        (CallFunction|StartRagdoll)
        (Utilities|FlowControl|Sequence
          (:then_0
            (Utilities|FlowControl|Delay 3.0)
            (Viewport|RemoveAllWidgets)
            (bind _returnvalue (UserInterface|CreateWidget "/Game/UI/Sequence_Widget_3.Sequence_Widget_3_C"))
            (UserInterface|Viewport|AddtoViewport _returnvalue 0)
            (bind _returnvalue_2 (UserInterface|CreateWidget "/Game/UI/Main_Menu/Main_FadeIN.Main_FadeIN_C"))
            (UserInterface|Viewport|AddtoViewport _returnvalue_2 0)
            (Input|SetInputModeUIOnly (Game|GetPlayerController 0) _returnvalue "LockAlways")
            (Pawn|Components|CharacterMovement|SetMovementMode (Variables|/Script/Engine.Character|GetCharacterMovement (Game|GetPlayerCharacter 0)) "MOVE_None" 0)
            (Utilities|FlowControl|Delay 1.0)
            (Game|OpenLevel(byName) "BossLevel_End"))
          (:then_1
            (bind _asplayer_controller (Utilities|Casting|CastToPlayer_Controller (Game|GetPlayerController 0)))
            (Default|NextLevel _asplayer_controller)))))))

(event Event경직끝
  ;[1 1 1] 경직
)

(event EventBaseMovement
  (Utilities|FlowControl|Delay 1.0)
  (CallFunction|CoolTime)
  (CallFunction|Chase))

(fn ConstructionScript
  (|CallParentFunction))

(fn 콜리전비활성화
  (bind _output_get (Variables|Default|SetCollision (Utilities|Array|MakeArray (Variables|Default|GetSwordCollision_R) (Variables|Default|GetSwordCollision_L) (Variables|Default|GetAttackRange))))
  (for _array_element _output_get
    (Collision|SetCollisionEnabled _array_element "NoCollision"))
  (Collision|SetCollisionEnabled (Variables|Default|GetSkillBody) "NoCollision")
  (return))