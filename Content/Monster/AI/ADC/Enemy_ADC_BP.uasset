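; Archer enemy child Blueprint that attaches a bow on BeginPlay and starts hunting MyEnemy after a short delay.
; Find moves into range with AIMoveTo, then loops a forward debug-drawn line trace.
; On a hit, a DoOnce-gated draw montage spawns Arrow_BP at its notify, resetting when the montage ends.
; On a miss, it snaps toward the target and, unless shooting, moves again with a distance-based acceptance radius.
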(event Custom|Find
  (bind _returnvalue (Transformation|GetActorLocation))
  (bind _returnvalue_2 (Transformation|GetActorLocation))
  (bind _returnvalue_3 (Transformation|GetActorLocation))
  (bind _returnvalue_4 (Transformation|GetActorTransform))
  (bind _returnvalue_5 (Transformation|GetActorLocation))
  (bind _my_enemy (Variables|Default|GetMy%20Enemy))
  (bind _my_enemy_2 (Variables|Default|GetMy%20Enemy))
  (bind _my_enemy_3 (Variables|Default|GetMy%20Enemy))
  (bind _returnvalue_6 (Transformation|GetActorLocation _my_enemy))
  (bind (_location _rotation) (Math|Transform|BreakTransform _returnvalue_4))
  (bind _returnvalue_7 (+ _returnvalue_5 "0, 0,25.000000"))
  (bind _returnvalue_8 (Math|Vector|Distance2D(Vector) _returnvalue_6 _returnvalue_2))
  (bind _returnvalue_9 (- _returnvalue_8 1e+02))
  (AI|AIMoveTo self "0.000000, 0,0.000000" (Variables|Default|GetMy%20Enemy) 8e+02 false
    (:OnSuccess
      (Utilities|FlowControl|DoOnce false
        (:Completed
          (bind _outhit (Collision|LineTraceByChannel _returnvalue_7 (+ _returnvalue_7 (* (Transformation|GetActorForwardVector) 10000)) "TraceTypeQuery3" false 0 "ForDuration" true "(R=1.000000,G=0.000000,B=0.000000,A=1.000000)" "(R=0.000000,G=1.000000,B=0.000000,A=1.000000)" 1.0 :!label _label))
          (if (== (.HitActor (Collision|BreakHitResult _outhit)) (Variables|Default|GetMy%20Enemy))
            (Utilities|FlowControl|DoOnce false :!label _label_2
              (:Completed
                (Variables|Default|SetisShoot true)
                (Animation|Montage|PlayMontage (Variables|Character|GetMesh) "/Game/Standing_Draw_Arrow_Montage.Standing_Draw_Arrow_Montage"
                  (:then
                    (goto _label))
                  (:OnCompleted
                    (Utilities|FlowControl|Sequence :!label _label_3
                      (:then_0
                        (goto _label_2 Reset))
                      (:then_1
                        (goto _label))))
                  (:OnInterrupted
                    (goto _label_3))
                  (:OnNotifyBegin
                    (Game|SpawnActorfromClass "/Game/Quever/Arrow_BP.Arrow_BP_C" (Math|Transform|MakeTransform (+ (* (Transformation|GetActorForwardVector) -5e+01) _location (* (Transformation|GetActorRightVector) 5e+01) (* (Transformation|GetActorUpVector) 15.0)) _rotation "2.000000,25.000000,25.000000") "AlwaysSpawn" 0 self)
                    (Variables|Default|SetisShoot false)))))
            (elif (Variables|Default|GetisShoot)
              (Utilities|IsValid _my_enemy_3
                (:Is%20Valid
                  (Transformation|SetActorLocationAndRotation _returnvalue (Math|Rotator|FindLookatRotation _returnvalue (Transformation|GetActorLocation _my_enemy_3)))
                  (goto _label)))
              (else
                (Utilities|IsValid _my_enemy_2
                  (:Is%20Valid
                    (Transformation|SetActorLocationAndRotation _returnvalue_3 (Math|Rotator|FindLookatRotation _returnvalue_3 (Transformation|GetActorLocation _my_enemy_2)))
                    (if (> _returnvalue_9 6e+02)
                      (AI|AIMoveTo self "0, 0, 0" (Variables|Default|GetMy%20Enemy) (Math|Float|Absolute(Float) _returnvalue_9) false
                        (:OnSuccess
                          (goto _label)))
                      (else
                        (AI|AIMoveTo self "0, 0, 0" (Variables|Default|GetMy%20Enemy) 6e+02 false
                          (:OnSuccess
                            (goto _label)))))))))))))))

(event Collision|EventActorBeginOverlap
  (params (OtherActor :type Actor%20Object%20Reference)))

(event EventBaseMovement)

(event EventBeginPlay
  (|CallParentFunction)
  (Utilities|FlowControl|Sequence
    (:then_0
      (bind _returnvalue (Game|SpawnActorfromClass "/Game/Monster/AI/Weapon/Enemy_Bow_Weapon.Enemy_Bow_Weapon_C" (Math|Transform|MakeTransform "0, 0, 0") "Undefined" 0 0))
      (bind _output_get (Variables|Default|SetEnemy_Weapon _returnvalue))
      (Transformation|AttachComponentToComponent _output_get (Variables|Character|GetMesh) "BowSocket" "SnapToTarget" "SnapToTarget" "SnapToTarget" true))
    (:then_1
      (Variables|Default|SetDistance 8e+02))
    (:then_2
      (Variables|Default|SetM_Inst "/Game/CityofBrass_Enemies/Materials/Corpse_Body_Inst2.Corpse_Body_Inst2")
      (Variables|Default|SetM_Clothes "/Game/CityofBrass_Enemies/Materials/Corpse_Clothes_Inst.Corpse_Clothes_Inst"))
    (:then_3
      (Utilities|FlowControl|Delay 1.0)
      (CallFunction|Find))))

(fn ConstructionScript
  (|CallParentFunction))