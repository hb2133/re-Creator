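; Warrior enemy Blueprint that spawns a weapon on its sword socket and fights its target in melee.
; AttackRange overlap loops the attack montage while the target stays in range, and SwordCollision_R deals damage gated by CanHitR.
; The stagger events (경직/경직끝) disable AttackRange, freeze a random damage-montage section at zero play rate with material flash, shake and sound, then play it out and re-enable attacking.
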(event OnComponentBeginOverlap(AttackRange)
  (params (OverlappedComponent :type Primitive%20Component%20Object%20Reference) (OtherActor :type Actor%20Object%20Reference) (OtherComp :type Primitive%20Component%20Object%20Reference) (OtherBodyIndex :type Integer) (bFromSweep :type Boolean) (SweepResult :type Hit%20Result%20Structure%20%28by%20ref%29))
  ;[1 1 1] AI
  (if (and (== OtherActor (Variables|Default|GetMy%20Enemy)) (not (Variables|Default|GetIsAttacking)))
    (Variables|Default|SetCanAttack true :!label _label)
    (Variables|Default|SetIsAttacking true :!label _label_2)
    (Animation|Montage|PlayMontage (Variables|Character|GetMesh) "/Game/Monster/AI/Corpse_Alert_Attack_Fast2_Montage.Corpse_Alert_Attack_Fast2_Montage"
      (:OnCompleted
        _)
      (:OnInterrupted
        _))
    (Variables|Default|SetIsAttacking false)
    (if (Math|Boolean|ANDBoolean (Variables|Default|GetCanAttack) (Variables|Default|GetIsAlive) (not (Variables|Default|GetisDamaged)))
      (goto _label_2)
      (else
        (Utilities|FlowControl|Delay 0.7)
        (if (stale OnComponentEndOverlap(AttackRange) _output_get)
          (goto _label))))))

(event OnComponentEndOverlap(AttackRange)
  (params (OverlappedComponent :type Primitive%20Component%20Object%20Reference) (OtherActor :type Actor%20Object%20Reference) (OtherComp :type Primitive%20Component%20Object%20Reference) (OtherBodyIndex :type Integer))
  ;[1 1 1] AI
  (if (and (== OtherActor (Variables|Default|GetMy%20Enemy)) (Variables|Default|GetCanAttack))
    (bind _output_get (Variables|Default|SetCanAttack false))))

(event OnComponentBeginOverlap(SwordCollision_R)
  (params (OverlappedComponent :type Primitive%20Component%20Object%20Reference) (OtherActor :type Actor%20Object%20Reference) (OtherComp :type Primitive%20Component%20Object%20Reference) (OtherBodyIndex :type Integer) (bFromSweep :type Boolean) (SweepResult :type Hit%20Result%20Structure%20%28by%20ref%29))
  ;[1 1 1] AI
  (if (and (== OtherActor (Variables|Default|GetMy%20Enemy)) (Variables|Default|GetCanHit_R))
    (Variables|Default|SetCanHit_R false)
    (Default|TakeDamage (Variables|Default|GetMy%20Enemy) 5.0)))

(event Event경직
  (params (DamageSize :type Float%20%28single-precision%29))
  (bind _mesh (Variables|Character|GetMesh))
  (bind _mesh_2 (Variables|Character|GetMesh))
  (Collision|SetCollisionEnabled (Variables|Default|GetAttackRange) "NoCollision")
  (CallFunction|GetDamage DamageSize)
  (Variables|Default|SetisDamaged true)
  (Components|Movement|StopMovementImmediately (Variables|Character|GetCharacterMovement))
  (Animation|Montage|PlayMontage (Variables|Character|GetMesh) "/Game/Monster/AI/Monster_Damaged.Monster_Damaged" 0.0 0.0 (Utilities|String|StringToName (Utilities|String|ToString(Integer) (Class|KismetMathLibrary|RandomIntegerfromStream 4 (Variables|Default|GetRandomAnimation))))
    (:then
      (Utilities|FlowControl|Sequence
        (:then_0
          (Rendering|Material|SetMaterial _mesh 0 (Variables|Default|GetM_Inst_Hit))
          (Rendering|Material|SetMaterial _mesh 1 (Variables|Default|GetM_Clothes_Hit))
          (Class|MatineeCameraShake|StartMatineeCameraShake (Game|GetPlayerCameraManager 0) "/Game/Camera/Shake.Shake_C" 0.05 "CameraLocal" "0, 0, 0")
          (Audio|PlaySound2D 0 1.0 1.0 0.0 0 0)
          (Audio|PlaySound2D 0 1.0 1.0 0.0 0 0))
        (:then_1
          (Utilities|FlowControl|Delay 0.3)
          (Rendering|Material|SetMaterial _mesh_2 0 (Variables|Default|GetM_Inst))
          (Rendering|Material|SetMaterial _mesh_2 1 (Variables|Default|GetM_Clothes)))))))

(event Collision|EventActorBeginOverlap
  (params (OtherActor :type Actor%20Object%20Reference)))

(event EventTick
  (params (DeltaSeconds :type Float%20%28single-precision%29)))

(event EventBeginPlay
  (|CallParentFunction)
  (Utilities|FlowControl|Sequence
    (:then_0
      (bind _returnvalue (Game|SpawnActorfromClass "/Game/Monster/AI/Weapon/Enemy_Weapon.Enemy_Weapon_C" (Math|Transform|MakeTransform "0, 0, 0") "Undefined" 0 0))
      (bind _output_get (Variables|Default|SetEnemy_Weapon _returnvalue))
      (Transformation|AttachComponentToComponent _output_get (Variables|Character|GetMesh) "SwordSocket" "SnapToTarget" "SnapToTarget" "SnapToTarget" true))
    (:then_1
      (Variables|Default|SetDistance 75.0))))

(event Event경직끝
  (Animation|Montage|PlayMontage (Variables|Character|GetMesh) "/Game/Monster/AI/Monster_Damaged.Monster_Damaged" 4.0 0.0 (Variables|Default|Getaction_Name)
    (:OnCompleted
      (Variables|Default|SetisDamaged false)
      (Collision|SetCollisionEnabled (Variables|Default|GetAttackRange) "QueryOnly"))))

(fn ConstructionScript
  (|CallParentFunction))