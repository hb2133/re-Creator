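; SpawnPoint_BP is a monster level spawn point actor that lifts itself clear of blocking objects when play begins.
; BeginPlay runs a short downward line trace for the configured object types, then loops, re-tracing and raising the actor in fixed steps until a trace finds no hit.
; Each pass traces before moving, so the actor still rises one step after the first clear trace.
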(event EventBeginPlay
  (bind _returnvalue (Transformation|GetActorLocation))
  (bind _returnvalue_2 (Transformation|GetActorLocation))
  (bind _returnvalue_3 (Transformation|GetActorLocation))
  (bind _returnvalue_4 (Collision|LineTraceForObjects (Transformation|GetActorLocation) (Math|Vector|MakeVector (.x _returnvalue_3) (.y _returnvalue_3) (+ (.z _returnvalue_3) -3e+01)) (Variables|Default|GetObject%20Types) false 0 "None"))
  (bind _output_get (Variables|Default|SetisCollision _returnvalue_4))
  (while _output_get
    (bind _returnvalue_5 (Collision|LineTraceForObjects (Transformation|GetActorLocation) (Math|Vector|MakeVector (.x _returnvalue) (.y _returnvalue) (+ (.z _returnvalue) -3e+01)) (Variables|Default|GetObject%20Types) false 0 "None"))
    (Variables|Default|SetisCollision _returnvalue_5)
    (Transformation|SetActorLocation (Math|Vector|MakeVector (.x _returnvalue_2) (.y _returnvalue_2) (+ (.z _returnvalue_2) 3e+01)) false false)))

(event Collision|EventActorBeginOverlap
  (params (OtherActor :type Actor%20Object%20Reference)))

(event EventTick
  (params (DeltaSeconds :type Float%20%28single-precision%29)))

(fn ConstructionScript)