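; Enemy spawner that spawns MonsterType actors after random delays, starting on BeginPlay or through ActivateSpawner.
; It spawns at its own transform or at a random SpawnPoint_BP matching its ID, slightly raised.
; Each spawn decrements Count, and once that runs out it calls SpawnOrderInsert on room managers and may keep looping.
; When IsClear is set after a spawn, it polls for zero remaining enemies and queries the managers' IsClearCheck.
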(event Custom|StartSpawning
  (Utilities|FlowControl|Delay (Math|Random|RandomFloatinRange (Variables|Default|GetSpawnDelay_Min) (Variables|Default|GetSpawnDelay_Max)) :!label _label)
  (if (not (Variables|Default|GetisClear))
    (if (Variables|Default|GetUseSpawnPoints)
      (if (== (Utilities|Array|Length (Variables|Default|GetSpawnPoints)) 1)
        (Variables|Default|SetSpawnLocation (Transformation|GetActorTransform (Utilities|Array|Get(acopy) (Variables|Default|GetSpawnPoints))))
        (else
          (Variables|Default|SetSpawnLocation (Transformation|GetActorTransform (Utilities|Array|Get(acopy) (Variables|Default|GetSpawnPoints) (Math|Random|RandomIntegerinRange 0 (- (Utilities|Array|Length (Variables|Default|GetSpawnPoints)) 1)))))))
      (else
        (Variables|Default|SetSpawnLocation (Transformation|GetActorTransform))))
    (Game|SpawnActorfromClass (Variables|Default|GetMonsterType) (Math|Transform|MakeTransform (+ (.location (Variables|Default|GetSpawnLocation)) "0, 0,3.000000") (.rotation (Variables|Default|GetSpawnLocation))) "AdjustIfPossibleButAlwaysSpawn" 0 0)
    (bind _output_get (Variables|Default|SetSpawntick (+ (Variables|Default|GetSpawntick) 1.0)))
    (Development|PrintString (Utilities|String|ToString(Float) _output_get))
    (if (< (Variables|Default|GetCount) -1)
      (goto _label)
      (else
        (Variables|Default|SetCount (- (Variables|Default|GetCount) 1))
        (if (> (Variables|Default|GetCount) 0)
          (goto _label)
          (elif (Variables|Default|GetisClear)
            (Utilities|FlowControl|Delay 1.0 :!label _label_2)
            (bind _outactors (Actor|GetAllActorsOfClass "/Game/Monster/AI/Parent/Enemy_BP.Enemy_BP_C"))
            (if (< (Utilities|Array|Length _outactors) 1)
              (bind _outactors_2 (Actor|GetAllActorsOfClass "/Game/Level/RoomManagerBP.RoomManagerBP_C"))
              (for _array_element _outactors_2
                (bind _isclear (Default|IsClearCheck _array_element))
                (if (not _isclear)
                  (goto _label_2)))
              (else
                (goto _label_2)))
            (else
              (bind _outactors_3 (Actor|GetAllActorsOfClass "/Game/Level/RoomManagerBP.RoomManagerBP_C"))
              (for _array_element_2 _outactors_3
                (Default|SpawnOrderInsert _array_element_2)
                (if (Variables|Default|GetisClear)
                  (goto _label_2)
                  (else
                    (goto _label)))))))))))

(event Custom|ActivateSpawner
  (CallFunction|StartSpawning))

(event EventBeginPlay
  (Utilities|FlowControl|Sequence
    (:then_0
      (if (Variables|Default|GetUseSpawnPoints)
        (bind _outactors (Actor|GetAllActorsOfClass "/Game/Monster/Levels/SpawnPoint_BP.SpawnPoint_BP_C"))
        (for _array_element _outactors
          (if (Utilities|Enum|Equal(Enum) (Variables|/Game/Monster/Levels/SpawnPoint_BP.SpawnPoint_BP_C|GetSpawnPoint_ID _array_element) (Variables|Default|GetSpawnPoints_ID))
            (Utilities|Array|AddUnique (Variables|Default|GetSpawnPoints) _array_element)))))
    (:then_1
      (if (Variables|Default|GetStartActive)
        (CallFunction|StartSpawning)))))

(fn ConstructionScript)