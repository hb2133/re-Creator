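; Base actor for a map partition that, on BeginPlay, clones gameplay markers attached to a referenced PivotActor onto itself.
; Attached actors are cast to spawn point, enemy spawner or room trigger, then respawned at their relative transform and attached to the partition.
; Cloned triggers are assigned to RoomTriggerDir slots by searching source object names for Up, Right or Left; no Down case is handled.
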(event EventBeginPlay
  (for _array_element (Actor|GetAttachedActors (Variables|Default|GetpivotActor) true)
    (Utilities|Array|Add (Variables|Default|Getmaps) _array_element))
  (for _array_element_2 (Variables|Default|Getmaps)
    (bind _asspawn_point_bp (Utilities|Casting|CastToSpawnPoint_BP _array_element_2)
      (:then
        (Development|PrintString "cast spawnPoint")
        (bind _returnvalue (Game|SpawnActorfromClass "/Game/Monster/Levels/SpawnPoint_BP.SpawnPoint_BP_C" (Transformation|GetRelativeTransform (Variables|/Script/Engine.Actor|GetRootComponent _asspawn_point_bp)) "AlwaysSpawn" 0 0))
        (Transformation|AttachActorToActor _returnvalue self "None" "KeepRelative" "SnapToTarget" "KeepRelative" true))
      (:CastFailed
        (bind _asenemy_spawner_bp (Utilities|Casting|CastToEnemy_Spawner_BP _array_element_2)
          (:then
            (Development|PrintString "cast spawner")
            (bind _returnvalue_2 (Game|SpawnActorfromClass "/Game/Monster/Levels/Enemy_Spawner_BP.Enemy_Spawner_BP_C" (Transformation|GetRelativeTransform (Variables|/Script/Engine.Actor|GetRootComponent _asenemy_spawner_bp)) "AlwaysSpawn" 0 0))
            (Transformation|AttachActorToActor _returnvalue_2 self "None" "KeepRelative" "SnapToTarget" "KeepRelative" true))
          (:CastFailed
            (bind _asroom_trigger (Utilities|Casting|CastToRoomTrigger _array_element_2))
            (Development|PrintString "cast Trigger")
            (bind _returnvalue_3 (Game|SpawnActorfromClass "/Game/Level/RoomTrigger.RoomTrigger_C" (Transformation|GetRelativeTransform (Variables|/Script/Engine.Actor|GetRootComponent _asroom_trigger)) "AlwaysSpawn" 0 0))
            (Transformation|AttachActorToActor _returnvalue_3 self "None" "KeepRelative" "SnapToTarget" "KeepRelative" true)
            (if (Utilities|String|Contains (Utilities|GetObjectName _asroom_trigger) "Up")
              (Variables|Default|SetroomTriggerDir (Utilities|Struct|MakeDirect _returnvalue_3 0 0 0))
              (elif (Utilities|String|Contains (Utilities|GetObjectName _asroom_trigger) "Right")
                (Variables|Default|SetroomTriggerDir (Utilities|Struct|MakeDirect 0 0 _returnvalue_3 0))
                (elif (Utilities|String|Contains (Utilities|GetObjectName _asroom_trigger) "Left")
                  (Variables|Default|SetroomTriggerDir (Utilities|Struct|MakeDirect 0 0 0 _returnvalue_3)))))))))))

(event Collision|EventActorBeginOverlap
  (params (OtherActor :type Actor%20Object%20Reference)))

(event EventTick
  (params (DeltaSeconds :type Float%20%28single-precision%29)))

(fn ConstructionScript)