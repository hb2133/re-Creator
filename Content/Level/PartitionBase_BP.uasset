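; Room partition actor that fills itself with a copy of a map template, self-building on BeginPlay only for the start room.
; InitRoomTrigger gets a random template from the level script, then clones its attached meshes, spawn points, enemy spawners, room manager and triggers onto itself.
; Trigger names set door directions, and the manager receives the room and spawner.
; Later calls rebuild contents from PivotActor, keeping triggers and manager; InitRoom is a separate rebuild variant.
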(event EventBeginPlay
  (if (Variables|Default|GetisStartRoom)
    (CallFunction|InitRoomTrigger)))

(event Collision|EventActorBeginOverlap
  (params (OtherActor :type Actor%20Object%20Reference)))

(event EventTick
  (params (DeltaSeconds :type Float%20%28single-precision%29)))

(fn ConstructionScript)

(fn InitRoom
  (bind _self self)
  (bind _self_2 self)
  (bind _roomdir (Variables|Default|GetroomDir))
  (bind _returnvalue (Utilities|GetObjectName _self))
  (Utilities|Array|Clear (Variables|Default|Getmaps))
  (bind _output_get (LocalVariables|SetMyAttachedActors (Actor|GetAttachedActors self true)))
  (for _array_element _output_get
    (Utilities|Casting|CastToRoomTrigger _array_element
      (:CastFailed
        (Utilities|Casting|CastToSpawnPoint_BP _array_element
          (:CastFailed
            (Utilities|Casting|CastToEnemy_Spawner_BP _array_element
              (:CastFailed
                (Utilities|Casting|CastToRoomManagerBP _array_element
                  (:CastFailed
                    (Actor|DestroyActor _array_element))))))))))
  (bind _output_get_2 (LocalVariables|SetMyAttachedActors (Actor|GetAttachedActors (Variables|Default|GetpivotActor) true)))
  (for _array_element_2 _output_get_2
    (if (Variables|Default|GetisInit)
      (Variables|Default|SetisInit true)
      (Utilities|Casting|CastToStaticMeshActor (LocalVariables|GetAttachElement))
      (Utilities|Array|Add (Variables|Default|Getmaps) (LocalVariables|GetAttachElement))
      (else
        (bind _output_get_3 (LocalVariables|SetAttachElement _array_element_2))
        (bind _asroom_trigger (Utilities|Casting|CastToRoomTrigger _output_get_3)
          (:then
            (Class|PartitionActor|AddTrigger _asroom_trigger)
            (Development|PrintString "cast Trigger")
            (Variables|Default|SetAs%20Room%20Trigger _asroom_trigger)
            (bind _returnvalue_2 (Game|SpawnActorfromClass "/Game/Level/RoomTrigger.RoomTrigger_C" (Transformation|GetRelativeTransform (Variables|/Script/Engine.Actor|GetRootComponent _asroom_trigger)) "AlwaysSpawn" 0 0))
            (bind _output_get_4 (Variables|Default|SetNewTrigger _returnvalue_2))
            (Transformation|AttachActorToActor _output_get_4 self "None" "KeepRelative" "SnapToTarget" "KeepRelative" true)
            (bind _returnvalue_3 (Class|PartitionActor|ContainName (Variables|Default|GetAs%20Room%20Trigger) "Up" "Down" "Right" "Left"))
            (Development|PrintString _returnvalue_3)
            (switch string _returnvalue_3
              (:Up
                (Class|PartitionActor|TriggerDirAdd (Variables|Default|GetNewTrigger) "UP")
                (Class|RoomTriggerBase|SetInfo (Variables|Default|GetNewTrigger) (Utilities|Struct|BreakDirect _roomdir))
                (Class|RoomTriggerBase|SetPartAct (Variables|Default|GetNewTrigger) (Variables|Default|GetAs%20Room%20Trigger)))
              (:Down
                (Class|PartitionActor|TriggerDirAdd (Variables|Default|GetNewTrigger) "DOWN")
                (Class|RoomTriggerBase|SetInfo (Variables|Default|GetNewTrigger) (Utilities|Struct|BreakDirect _roomdir))
                (Class|RoomTriggerBase|SetPartAct (Variables|Default|GetNewTrigger) (Variables|Default|GetAs%20Room%20Trigger)))
              (:Right
                (Class|PartitionActor|TriggerDirAdd (Variables|Default|GetNewTrigger) "RIGHT")
                (Class|RoomTriggerBase|SetInfo (Variables|Default|GetNewTrigger) (Utilities|Struct|BreakDirect _roomdir))
                (Class|RoomTriggerBase|SetPartAct (Variables|Default|GetNewTrigger) (Variables|Default|GetAs%20Room%20Trigger)))
              (:Left
                (Class|PartitionActor|TriggerDirAdd (Variables|Default|GetNewTrigger) "LEFT")
                (Class|RoomTriggerBase|SetInfo (Variables|Default|GetNewTrigger) (Utilities|Struct|BreakDirect _roomdir))
                (Class|RoomTriggerBase|SetPartAct (Variables|Default|GetNewTrigger) (Variables|Default|GetAs%20Room%20Trigger))))
            (if (Variables|Default|GetisStartRoom)
              (Variables|/Game/Level/RoomTrigger.RoomTrigger_C|SetisUsed (Variables|Default|GetNewTrigger) false)
              (else
                (Variables|/Game/Level/RoomTrigger.RoomTrigger_C|SetisUsed (Variables|Default|GetNewTrigger) true)))
            (Variables|Default|SetisInit true))
          (:CastFailed
            (bind _asspawn_point_bp (Utilities|Casting|CastToSpawnPoint_BP (LocalVariables|GetAttachElement))
              (:then
                (Class|PartitionActor|AddTrigger _asspawn_point_bp)
                (Development|PrintString "cast spawnPoint")
                (bind _returnvalue_4 (Game|SpawnActorfromClass "/Game/Monster/Levels/SpawnPoint_BP.SpawnPoint_BP_C" (Transformation|GetRelativeTransform (Variables|/Script/Engine.Actor|GetRootComponent _asspawn_point_bp)) "AlwaysSpawn" 0 0))
                (Transformation|AttachActorToActor _returnvalue_4 self "None" "KeepRelative" "SnapToTarget" "KeepRelative" true)
                (Variables|/Game/Monster/Levels/SpawnPoint_BP.SpawnPoint_BP_C|SetSpawnPoint_ID _returnvalue_4 _returnvalue))
              (:CastFailed
                (bind _asenemy_spawner_bp (Utilities|Casting|CastToEnemy_Spawner_BP (LocalVariables|GetAttachElement))
                  (:then
                    (Class|PartitionActor|AddTrigger _asenemy_spawner_bp)
                    (Development|PrintString "cast spawner")
                    (bind _returnvalue_5 (Game|SpawnActorfromClass "/Game/Monster/Levels/Enemy_Spawner_BP.Enemy_Spawner_BP_C" (Transformation|GetRelativeTransform (Variables|/Script/Engine.Actor|GetRootComponent _asenemy_spawner_bp)) "AlwaysSpawn" 0 0))
                    (Transformation|AttachActorToActor _returnvalue_5 self "None" "KeepRelative" "SnapToTarget" "KeepRelative" true)
                    (bind _output_get_5 (Variables|/Game/Monster/Levels/Enemy_Spawner_BP.Enemy_Spawner_BP_C|SetSpawnPoints_ID _returnvalue_5 _returnvalue))
                    (Variables|/Game/Monster/Levels/Enemy_Spawner_BP.Enemy_Spawner_BP_C|SetActivation_ID _returnvalue_5 _output_get_5))
                  (:CastFailed
                    (bind _asroom_manager_bp (Utilities|Casting|CastToRoomManagerBP (LocalVariables|GetAttachElement))
                      (:then
                        (Class|PartitionActor|AddTrigger _asroom_manager_bp)
                        (Development|PrintString "cast Manager")
                        (bind _returnvalue_6 (Game|SpawnActorfromClass "/Game/Level/RoomManagerBP.RoomManagerBP_C" (Transformation|GetRelativeTransform (Variables|/Script/Engine.Actor|GetRootComponent _asroom_manager_bp)) "AlwaysSpawn" 0 0))
                        (bind _output_get_6 (Variables|Default|SetNewRoomManager _returnvalue_6))
                        (Transformation|AttachActorToActor _output_get_6 _self_2 "None" "KeepRelative" "SnapToTarget" "KeepRelative" true)
                        (Variables|/Script/test_Project_3.RoomManager|SetPartitionActor _output_get_6 _self_2)
                        (Class|RoomManager|SetInfoRoom _output_get_6 _self_2))
                      (:CastFailed
                        (Utilities|FlowControl|Sequence
                          (:then_0
                            (Utilities|Array|Add (Variables|Default|Getmaps) (LocalVariables|GetAttachElement)))
                          (:then_1
                            (Class|PartitionActor|SetRoom)
                            (Class|RoomManager|SetInfoRoom (Variables|Default|GetNewRoomManager) self)
                            (Variables|Default|SetisInit true))))))))))))))
  (for _array_element_3 (Variables|Default|Getmaps)
    (bind _asstatic_mesh_actor (Utilities|Casting|CastToStaticMeshActor _array_element_3))
    (Development|PrintString "cast staticmesh")
    (bind _returnvalue_7 (Game|SpawnActorfromClass "/Script/Engine.StaticMeshActor" (Transformation|GetRelativeTransform (Variables|/Script/Engine.Actor|GetRootComponent _asstatic_mesh_actor)) "AlwaysSpawn" 0 0))
    (Transformation|SetMobility _returnvalue_7 "Movable")
    (Transformation|AttachActorToActor _returnvalue_7 self "None" "KeepRelative" "SnapToTarget" "KeepRelative" true)
    (Components|StaticMesh|SetStaticMesh (Variables|/Script/Engine.StaticMeshActor|GetStaticMeshComponent _returnvalue_7) (Variables|/Script/Engine.StaticMeshComponent|GetStaticMesh (Variables|/Script/Engine.StaticMeshActor|GetStaticMeshComponent _asstatic_mesh_actor))))
  (bind _asmap_template_bp (Utilities|Casting|CastToMapTemplateBP (Variables|Default|GetpivotActor)))
  (Variables|Default|SetroomTriggerDir (Utilities|Struct|MakeDirect (.up (Variables|Default|GetroomTriggerDir)) (.down (Variables|Default|GetroomTriggerDir)) (.right (Variables|Default|GetroomTriggerDir)) (.left (Variables|Default|GetroomTriggerDir)) (.current (Variables|/Script/test_Project_3.PartitionActor|GetroomDir _asmap_template_bp)))))

(fn InitRoomTrigger
  (bind _self self)
  (bind _self_2 self)
  (bind _self_3 self)
  (bind _maps (Variables|Default|Getmaps))
  (bind _roomdir (Variables|Default|GetroomDir))
  (bind _returnvalue (Utilities|GetObjectName _self_2))
  (bind _returnvalue_2 (Utilities|GetObjectName _self))
  (if (Variables|Default|GetisInit)
    ;[1 1 1] managerInit이후
    (for _array_element _maps
      (Actor|DestroyActor _array_element))
    (Utilities|Array|Clear _maps)
    (for _array_element_2 (Actor|GetAttachedActors (Variables|Default|GetpivotActor) true)
      (LocalVariables|SetAttachElement _array_element_2)
      (Utilities|FlowControl|Sequence
        (:then_0
          (bind _asstatic_mesh_actor (Utilities|Casting|CastToStaticMeshActor (LocalVariables|GetAttachElement)))
          (Development|PrintString "cast staticmesh")
          (bind _returnvalue_3 (Game|SpawnActorfromClass "/Script/Engine.StaticMeshActor" (Transformation|GetRelativeTransform (Variables|/Script/Engine.Actor|GetRootComponent _asstatic_mesh_actor)) "AlwaysSpawn" 0 0))
          (Transformation|SetMobility _returnvalue_3 "Movable")
          (Transformation|AttachActorToActor _returnvalue_3 self "None" "KeepRelative" "SnapToTarget" "KeepRelative" true)
          (Components|StaticMesh|SetStaticMesh (Variables|/Script/Engine.StaticMeshActor|GetStaticMeshComponent _returnvalue_3) (Variables|/Script/Engine.StaticMeshComponent|GetStaticMesh (Variables|/Script/Engine.StaticMeshActor|GetStaticMeshComponent _asstatic_mesh_actor)))
          (Utilities|Array|Add (Variables|Default|Getmaps) _returnvalue_3))
        (:then_1
          (bind _asspawn_point_bp (Utilities|Casting|CastToSpawnPoint_BP (LocalVariables|GetAttachElement)))
          (Development|PrintString "cast spawnPoint")
          (bind _returnvalue_4 (Game|SpawnActorfromClass "/Game/Monster/Levels/SpawnPoint_BP.SpawnPoint_BP_C" (Transformation|GetRelativeTransform (Variables|/Script/Engine.Actor|GetRootComponent _asspawn_point_bp)) "AlwaysSpawn" 0 0))
          (Transformation|AttachActorToActor _returnvalue_4 self "None" "KeepRelative" "SnapToTarget" "KeepRelative" true)
          (Variables|/Game/Monster/Levels/SpawnPoint_BP.SpawnPoint_BP_C|SetSpawnPoint_ID _returnvalue_4 _returnvalue_2)
          (Utilities|Array|Add (Variables|Default|Getmaps) _returnvalue_4))
        (:then_2
          (bind _asenemy_spawner_bp (Utilities|Casting|CastToEnemy_Spawner_BP (LocalVariables|GetAttachElement)))
          (Development|PrintString "cast spawner")
          (bind _returnvalue_5 (Game|SpawnActorfromClass "/Game/Monster/Levels/Enemy_Spawner_BP.Enemy_Spawner_BP_C" (Transformation|GetRelativeTransform (Variables|/Script/Engine.Actor|GetRootComponent _asenemy_spawner_bp)) "AlwaysSpawn" 0 0))
          (Transformation|AttachActorToActor _returnvalue_5 self "None" "KeepRelative" "SnapToTarget" "KeepRelative" true)
          (bind _output_get (Variables|/Game/Monster/Levels/Enemy_Spawner_BP.Enemy_Spawner_BP_C|SetSpawnPoints_ID _returnvalue_5 _returnvalue_2))
          (Variables|/Game/Monster/Levels/Enemy_Spawner_BP.Enemy_Spawner_BP_C|SetActivation_ID _returnvalue_5 _output_get)
          (Utilities|Array|Add (Variables|Default|Getmaps) _returnvalue_5)
          (Variables|/Game/Level/RoomManagerBP.RoomManagerBP_C|SetmyEnemySpawner (Variables|Default|GetNewRoomManager) _returnvalue_5))))
    (elif (not (> (Utilities|Array|Length (Variables|Default|GetTriggers)) 0))
      (bind _returnvalue_6 (Actor|GetActorOfClass "/Script/test_Project_3.MyLevelScriptActor"))
      (bind _returnvalue_7 (Class|MyLevelScriptActor|RandomMapTemplate _returnvalue_6))
      (Variables|Default|SetpivotActor _returnvalue_7)
      ;[1 1 1] managerInit이전
      (for _array_element_3 (Actor|GetAttachedActors _returnvalue_7 true)
        (LocalVariables|SetAttachElement _array_element_3)
        (Utilities|FlowControl|Sequence
          (:then_0
            (bind _asroom_trigger (Utilities|Casting|CastToRoomTrigger (LocalVariables|GetAttachElement)))
            (Class|PartitionActor|AddTrigger _asroom_trigger)
            (Development|PrintString "cast Trigger")
            (Variables|Default|SetAs%20Room%20Trigger _asroom_trigger)
            (bind _returnvalue_8 (Game|SpawnActorfromClass "/Game/Level/RoomTrigger.RoomTrigger_C" (Transformation|GetRelativeTransform (Variables|/Script/Engine.Actor|GetRootComponent _asroom_trigger)) "AlwaysSpawn" 0 0))
            (bind _output_get_2 (Variables|Default|SetNewTrigger _returnvalue_8))
            (Transformation|AttachActorToActor _output_get_2 self "None" "KeepRelative" "SnapToTarget" "KeepRelative" true)
            (bind _returnvalue_9 (Class|PartitionActor|ContainName (Variables|Default|GetAs%20Room%20Trigger) "Up" "Down" "Right" "Left"))
            (Development|PrintString _returnvalue_9)
            (switch string _returnvalue_9
              (:Up
                (Class|PartitionActor|TriggerDirAdd (Variables|Default|GetNewTrigger) "UP")
                (Class|RoomTriggerBase|SetInfo (Variables|Default|GetNewTrigger) (Utilities|Struct|BreakDirect _roomdir))
                (Class|RoomTriggerBase|SetPartAct (Variables|Default|GetNewTrigger) (Variables|Default|GetAs%20Room%20Trigger)))
              (:Down
                (Class|PartitionActor|TriggerDirAdd (Variables|Default|GetNewTrigger) "DOWN")
                (Class|RoomTriggerBase|SetInfo (Variables|Default|GetNewTrigger) (Utilities|Struct|BreakDirect _roomdir))
                (Class|RoomTriggerBase|SetPartAct (Variables|Default|GetNewTrigger) (Variables|Default|GetAs%20Room%20Trigger)))
              (:Right
                (Class|PartitionActor|TriggerDirAdd (Variables|Default|GetNewTrigger) "RIGHT")
                (Class|RoomTriggerBase|SetInfo (Variables|Default|GetNewTrigger) (Utilities|Struct|BreakDirect _roomdir))
                (Class|RoomTriggerBase|SetPartAct (Variables|Default|GetNewTrigger) (Variables|Default|GetAs%20Room%20Trigger)))
              (:Left
                (Class|PartitionActor|TriggerDirAdd (Variables|Default|GetNewTrigger) "LEFT")
                (Class|RoomTriggerBase|SetInfo (Variables|Default|GetNewTrigger) (Utilities|Struct|BreakDirect _roomdir))
                (Class|RoomTriggerBase|SetPartAct (Variables|Default|GetNewTrigger) (Variables|Default|GetAs%20Room%20Trigger))))
            (if (Variables|Default|GetisStartRoom)
              (Variables|/Game/Level/RoomTrigger.RoomTrigger_C|SetisUsed (Variables|Default|GetNewTrigger) false)
              (else
                (Variables|/Game/Level/RoomTrigger.RoomTrigger_C|SetisUsed (Variables|Default|GetNewTrigger) true)))
            (Variables|Default|SetisInit true))
          (:then_1
            (bind _asspawn_point_bp_2 (Utilities|Casting|CastToSpawnPoint_BP (LocalVariables|GetAttachElement)))
            (Development|PrintString "cast spawnPoint")
            (bind _returnvalue_10 (Game|SpawnActorfromClass "/Game/Monster/Levels/SpawnPoint_BP.SpawnPoint_BP_C" (Transformation|GetRelativeTransform (Variables|/Script/Engine.Actor|GetRootComponent _asspawn_point_bp_2)) "AlwaysSpawn" 0 0))
            (Transformation|AttachActorToActor _returnvalue_10 self "None" "KeepRelative" "SnapToTarget" "KeepRelative" true)
            (Variables|/Game/Monster/Levels/SpawnPoint_BP.SpawnPoint_BP_C|SetSpawnPoint_ID _returnvalue_10 _returnvalue)
            (Utilities|Array|Add (Variables|Default|Getmaps) _returnvalue_10))
          (:then_2
            (bind _asenemy_spawner_bp_2 (Utilities|Casting|CastToEnemy_Spawner_BP (LocalVariables|GetAttachElement)))
            (Development|PrintString "cast spawner")
            (bind _returnvalue_11 (Game|SpawnActorfromClass "/Game/Monster/Levels/Enemy_Spawner_BP.Enemy_Spawner_BP_C" (Transformation|GetRelativeTransform (Variables|/Script/Engine.Actor|GetRootComponent _asenemy_spawner_bp_2)) "AlwaysSpawn" 0 0))
            (Transformation|AttachActorToActor _returnvalue_11 self "None" "KeepRelative" "SnapToTarget" "KeepRelative" true)
            (bind _output_get_3 (Variables|/Game/Monster/Levels/Enemy_Spawner_BP.Enemy_Spawner_BP_C|SetSpawnPoints_ID _returnvalue_11 _returnvalue))
            (Variables|/Game/Monster/Levels/Enemy_Spawner_BP.Enemy_Spawner_BP_C|SetActivation_ID _returnvalue_11 _output_get_3)
            (Utilities|Array|Add (Variables|Default|Getmaps) _returnvalue_11))
          (:then_3
            (bind _asroom_manager_bp (Utilities|Casting|CastToRoomManagerBP (LocalVariables|GetAttachElement)))
            (Class|PartitionActor|AddTrigger _asroom_manager_bp)
            (Development|PrintString "cast Manager")
            (bind _returnvalue_12 (Game|SpawnActorfromClass "/Game/Level/RoomManagerBP.RoomManagerBP_C" (Transformation|GetRelativeTransform (Variables|/Script/Engine.Actor|GetRootComponent _asroom_manager_bp)) "AlwaysSpawn" 0 0))
            (bind _output_get_4 (Variables|Default|SetNewRoomManager _returnvalue_12))
            (Transformation|AttachActorToActor _output_get_4 _self_3 "None" "KeepRelative" "SnapToTarget" "KeepRelative" true)
            (Variables|/Script/test_Project_3.RoomManager|SetPartitionActor _output_get_4 _self_3)
            (Class|RoomManager|SetInfoRoom _output_get_4 _self_3))
          (:then_4
            (bind _asstatic_mesh_actor_2 (Utilities|Casting|CastToStaticMeshActor (LocalVariables|GetAttachElement)))
            (Development|PrintString "cast staticmesh")
            (bind _returnvalue_13 (Game|SpawnActorfromClass "/Script/Engine.StaticMeshActor" (Transformation|GetRelativeTransform (Variables|/Script/Engine.Actor|GetRootComponent _asstatic_mesh_actor_2)) "AlwaysSpawn" 0 0))
            (Transformation|SetMobility _returnvalue_13 "Movable")
            (Transformation|AttachActorToActor _returnvalue_13 self "None" "KeepRelative" "SnapToTarget" "KeepRelative" true)
            (Components|StaticMesh|SetStaticMesh (Variables|/Script/Engine.StaticMeshActor|GetStaticMeshComponent _returnvalue_13) (Variables|/Script/Engine.StaticMeshComponent|GetStaticMesh (Variables|/Script/Engine.StaticMeshActor|GetStaticMeshComponent _asstatic_mesh_actor_2)))
            (Utilities|Array|Add (Variables|Default|Getmaps) _returnvalue_13))))
      (Class|PartitionActor|SetRoom)
      (Class|RoomManager|SetInfoRoom (Variables|Default|GetNewRoomManager) self)
      (Variables|Default|SetisInit true)
      (Class|PartitionActor|SetNextMap (Variables|Default|GetroomDir) (Variables|Default|GetroomTriggerDir))
      (Variables|/Game/Level/RoomManagerBP.RoomManagerBP_C|SetmyEnemySpawner (Variables|Default|GetNewRoomManager) _returnvalue_11))))

(fn DuplicateMesh)