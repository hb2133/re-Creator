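; RoomDoorBP is a room door that raises its static mesh when a room is cleared and lowers it when a room initializes.
; RoomClear plays the OpenDoor timeline if the mesh is down, but doors flagged IsSide ignore the first call after a reset, using FirstAccept.
; RoomInit clears that flag and plays CloseDoor if the mesh is raised.
; Both timelines apply Z offsets to a cached relative location.
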(event EventBeginPlay)

(event Collision|EventActorBeginOverlap
  (params (OtherActor :type Actor%20Object%20Reference)))

(event EventTick
  (params (DeltaSeconds :type Float%20%28single-precision%29)))

(event EventRoomClear
  (bind _staticmesh (Variables|Default|GetStaticMesh))
  (bind _relativelocation (Variables|/Script/Engine.SceneComponent|GetRelativeLocation _staticmesh))
  (if (Variables|Default|GetisSide)
    (if (Variables|Default|GetfirstAccept)
      (if (<= (.Z (Math|Vector|BreakVector _relativelocation)) 0.0) :!label _label
        (bind _output_get (Variables|Default|SetRelative%20Location _relativelocation))
        (bind _새_트랙_0 (Timeline|openDoor Play)
          (:Update
            (Transformation|SetRelativeLocation _staticmesh (+ _output_get (Math|Vector|MakeVector 0.0 0.0 _새_트랙_0)) false false))))
      (else
        (Variables|Default|SetfirstAccept true)))
    (else
      (goto _label))))

(event EventRoomInit
  (bind _staticmesh (Variables|Default|GetStaticMesh))
  (bind _relativelocation (Variables|/Script/Engine.SceneComponent|GetRelativeLocation _staticmesh))
  (Variables|Default|SetfirstAccept false)
  (if (> (.Z (Math|Vector|BreakVector _relativelocation)) 0.0)
    (bind _output_get (Variables|Default|SetRelative%20Location _relativelocation))
    (bind _새_트랙_0 (Timeline|closeDoor Play)
      (:Update
        (Transformation|SetRelativeLocation _staticmesh (- _output_get (Math|Vector|MakeVector 0.0 0.0 _새_트랙_0)) false false)))))

(fn ConstructionScript)