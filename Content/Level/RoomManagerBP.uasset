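; Per-room manager actor that runs a room's battle, from monster spawning to clear detection.
; On the character's call while the player is inside its box, it hides its mesh, starts the spawner matching its parent actor's name and feeds it queued monsters.
; Tick declares a clear when no enemies exist anywhere and the queue is empty.
; Battle start resets left and right neighbor rooms; clearing restores the mesh and resets next-room triggers.
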(event OnComponentBeginOverlap(Box)
  (params (OverlappedComponent :type Primitive%20Component%20Object%20Reference) (OtherActor :type Actor%20Object%20Reference) (OtherComp :type Primitive%20Component%20Object%20Reference) (OtherBodyIndex :type Integer) (bFromSweep :type Boolean) (SweepResult :type Hit%20Result%20Structure%20%28by%20ref%29))
  (Utilities|Casting|CastToThirdPersonCharacter OtherActor)
  (Variables|Default|SetCurrentRoom true))

(event OnComponentEndOverlap(Box)
  (params (OverlappedComponent :type Primitive%20Component%20Object%20Reference) (OtherActor :type Actor%20Object%20Reference) (OtherComp :type Primitive%20Component%20Object%20Reference) (OtherBodyIndex :type Integer))
  (Variables|Default|SetCurrentRoom false))

(event Custom|ActivateSpawner
  (params (Activation_ID :type String))
  ;[1 1 1] 스폰
  (bind _outactors (Actor|GetAllActorsOfClass "/Game/Monster/Levels/Enemy_Spawner_BP.Enemy_Spawner_BP_C"))
  (bind _array_element (Utilities|Array|ForEachLoopwithBreak _outactors :!label _label)
    (:LoopBody
      (if (Utilities|Enum|Equal(Enum) (Variables|/Game/Monster/Levels/Enemy_Spawner_BP.Enemy_Spawner_BP_C|GetActivation_ID _array_element) Activation_ID)
        (goto _label Break)))
    (:Completed
      (Utilities|FlowControl|DoOnce false
        (:Completed
          (Default|StartSpawning _array_element))))))

(event Custom|RoomManagerCall_Event_0
  ;[1 1 1] 몬스터스폰콜
  (if (Variables|Default|GetCurrentRoom)
    (if (not (Variables|Default|GetisPlaying))
      (CallFunction|ActivateSpawner (Utilities|GetObjectName (Actor|GetAttachParentActor)))
      (Variables|Default|SetisPlaying true)
      (Rendering|SetActorHiddenInGame true)
      (Collision|SetCollisionEnabled (Variables|Default|GetStaticMesh) "NoCollision")
      (Default|CallRoomBattleStart)
      (CallFunction|SpawnOrderInsert))))

(event Custom|RoomBattleStart_Event
  (bind _partitionactor (Variables|Default|GetPartitionActor))
  (bind _roomdir (Variables|/Script/test_Project_3.PartitionActor|GetroomDir _partitionactor))
  (bind (_up _down _right _left) (Utilities|Struct|BreakDirect _roomdir))
  ;[1 1 1] 전투시작 이벤트
  (bind _aspartition_base_bp (Utilities|Casting|CastToPartitionBase_BP (.nextMap (Utilities|Struct|BreakRoomNode _right))))
  (Default|InitRoomTrigger _aspartition_base_bp)
  (bind _aspartition_base_bp_2 (Utilities|Casting|CastToPartitionBase_BP (.nextMap (Utilities|Struct|BreakRoomNode _left))))
  (Default|InitRoomTrigger _aspartition_base_bp_2)
  (CallFunction|Init (Variables|/Game/Level/PartitionBase_BP.PartitionBase_BP_C|GetNewRoomManager _aspartition_base_bp))
  (CallFunction|Init (Variables|/Game/Level/PartitionBase_BP.PartitionBase_BP_C|GetNewRoomManager _aspartition_base_bp_2)))

(event Custom|RoomClearCall
  (bind _inforoom (Variables|Default|GetInfoRoom))
  (bind _partitionactor (Variables|Default|GetPartitionActor))
  (bind (_up _down _right _left) (Utilities|Struct|BreakDirect _inforoom))
  (bind _roomdir (Variables|/Script/test_Project_3.PartitionActor|GetroomDir _partitionactor))
  (bind (_up_2 _down_2 _right_2 _left_2) (Utilities|Struct|BreakDirect _roomdir))
  ;[1 1 1] 클리어콜
  (bind _asroom_trigger (Utilities|Casting|CastToRoomTrigger (.nextMapTrigger (Utilities|Struct|BreakRoomNode _up))))
  (Variables|/Game/Level/RoomTrigger.RoomTrigger_C|SetisUsed _asroom_trigger false)
  (bind _asroom_trigger_2 (Utilities|Casting|CastToRoomTrigger (.nextMapTrigger (Utilities|Struct|BreakRoomNode _right))))
  (Variables|/Game/Level/RoomTrigger.RoomTrigger_C|SetisUsed _asroom_trigger_2 false)
  (bind _asroom_trigger_3 (Utilities|Casting|CastToRoomTrigger (.nextMapTrigger (Utilities|Struct|BreakRoomNode _left))))
  (Variables|/Game/Level/RoomTrigger.RoomTrigger_C|SetisUsed _asroom_trigger_3 false)
  (Rendering|SetActorHiddenInGame false)
  (Collision|SetCollisionEnabled (Variables|Default|GetStaticMesh) "QueryAndPhysics")
  (bind _aspartition_base_bp (Utilities|Casting|CastToPartitionBase_BP (.nextMap (Utilities|Struct|BreakRoomNode _right_2))))
  (Variables|RoomManagerBP_C|SetisPlaying (Variables|/Game/Level/PartitionBase_BP.PartitionBase_BP_C|GetNewRoomManager _aspartition_base_bp) false)
  (bind _aspartition_base_bp_2 (Utilities|Casting|CastToPartitionBase_BP (.nextMap (Utilities|Struct|BreakRoomNode _left_2))))
  (Variables|RoomManagerBP_C|SetisPlaying (Variables|/Game/Level/PartitionBase_BP.PartitionBase_BP_C|GetNewRoomManager _aspartition_base_bp_2) false)
  (Variables|Default|SetisClear true))

(event Custom|Init
  (Variables|Default|SetisClear false)
  (Variables|Default|SetCurrentRoom false)
  (Variables|Default|SetisPlaying false))

(event Custom|SpawnOrderInsert
  (bind _roomstatus (Variables|Default|GetRoomStatus))
  (bind _myenemyspawner (Variables|Default|GetmyEnemySpawner))
  (bind _currentmonsters (Utilities|Struct|BreakRoomStatus _roomstatus))
  (bind _output (Utilities|Array|Get(acopy) _currentmonsters))
  (bind (_count _cost _enemyclass) (Utilities|Struct|BreakSpawnOrder _output))
  (if (not (== _myenemyspawner 0))
    (if (> (Utilities|Array|Length _currentmonsters) 0)
      (bind _asactor (Utilities|Casting|CastToActorClass _enemyclass))
      (Development|PrintString (Utilities|String|ToString(Integer) (stale _output_get)))
      (Variables|/Game/Monster/Levels/Enemy_Spawner_BP.Enemy_Spawner_BP_C|SetMonsterType _myenemyspawner _asactor)
      (bind _output_get (Variables|/Game/Monster/Levels/Enemy_Spawner_BP.Enemy_Spawner_BP_C|SetCount _myenemyspawner _count))
      (Utilities|Array|RemoveItem _currentmonsters _output)
      (else
        (CallFunction|RoomClearCall)
        (Variables|/Game/Monster/Levels/Enemy_Spawner_BP.Enemy_Spawner_BP_C|SetisClear (Variables|Default|GetmyEnemySpawner) true)))))

(event EventBeginPlay
  (Class|RoomManager|RandomEnemyOrder)
  (bind _asthird_person_character (Utilities|Casting|CastToThirdPersonCharacter (Game|GetPlayerCharacter 0)))
  ;[1 1 1] 몬스터스폰콜
  (EventDispatchers|AssignRoomManagerCall _asthird_person_character (delegate Custom|RoomManagerCall_Event_0))
  ;[1 1 1] 전투시작 이벤트
  (EventDispatchers|BindEventtoRoomBattleStart (delegate Custom|RoomBattleStart_Event)))

(event Collision|EventActorBeginOverlap
  (params (OtherActor :type Actor%20Object%20Reference)))

(event EventTick
  (params (DeltaSeconds :type Float%20%28single-precision%29))
  (bind _roomstatus (Variables|Default|GetRoomStatus))
  (bind _returnvalue (Utilities|Array|Length (.currentmonsters _roomstatus)))
  ;[1 1 1] 클리어판단
  (if (Variables|Default|GetisPlaying)
    (bind _outactors (Actor|GetAllActorsOfClass "/Game/Monster/AI/Parent/Enemy_BP.Enemy_BP_C"))
    (Development|PrintString (Utilities|String|ToString(Integer) (Utilities|Array|Length _outactors)))
    (Development|PrintString (Utilities|String|ToString(Integer) _returnvalue))
    (if (and (< (Utilities|Array|Length _outactors) 1) (< _returnvalue 1))
      (Variables|Default|SetisPlaying false)
      (CallFunction|RoomClearCall))))

(fn ConstructionScript)